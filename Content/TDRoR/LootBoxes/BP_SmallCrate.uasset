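; BP_SmallCrate is a lootable crate that pays out currency, built on looting logic from the C++ LootCrate.
; A box trigger flags when a TwinStickPawn is in open range and shows an interact widget while the crate is unopened.
; CheckLooted, if loot has not been given, calls the native Loot function, swaps the cube to an orange material and sends the result to the GameInstance for a currency-gain UI message.
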(event `self.ReceiveTick`
  (params (DeltaSeconds :type "Float (single-precision)")))

(event `CheckLooted`
  ;[1 1 1] Check if looted already, if not loot box
  (if (not (`self.givenLoot`))
    ;[1 1 1] Looting Function
    ;;[1 1 1] From LootCrate.cpp
    (bind _returnvalue (`self.Loot`))
    ;;[1 1 1] Change the Chest Mesh
    (`PrimitiveComponent.SetMaterial` (`self.Cube`) 0 "/Game/TwinStick/Meshes/OrangeMaterial.OrangeMaterial")
    ;;[1 1 1] For UI Elements
    (message `/Game/TDRoR/LootBoxes/BPI_Interact.Gain Currency Event` (`GameplayStatics.GetGameInstance`) _returnvalue)))

(event `self.Box.OnComponentBeginOverlap`
  (params (OverlappedComponent :type "PrimitiveComponent Object Reference") (OtherActor :type "Actor Object Reference") (OtherComp :type "PrimitiveComponent Object Reference") (OtherBodyIndex :type Integer) (bFromSweep :type Boolean) (SweepResult :type "HitResult Structure (by ref)"))
  ;[1 1 1] Interact Widget
  (cast `/Game/TwinStickBP/Blueprints/TwinStickPawn` OtherActor)
  (if (not (`self.opened`))
    (set `self.inOpenRange` true)
    (`SceneComponent.SetVisibility` (`self.Widget`) true false)))

(event `self.Box.OnComponentEndOverlap`
  (params (OverlappedComponent :type "PrimitiveComponent Object Reference") (OtherActor :type "Actor Object Reference") (OtherComp :type "PrimitiveComponent Object Reference") (OtherBodyIndex :type Integer))
  ;[1 1 1] Interact Widget
  (cast `/Game/TwinStickBP/Blueprints/TwinStickPawn` OtherActor)
  (if (`self.opened`)
    _
    (else
      _))
  (set `self.inOpenRange` false)
  (`SceneComponent.SetVisibility` (`self.Widget`) false false))

(fn `UserConstructionScript`
  (`SceneComponent.SetVisibility` (`self.Widget`) false false))