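; Master item pickup that modifies the player's health, damage or fire rate, chosen by its Stat variable.
; When a TwinStickPawn overlaps the mesh, it reads that stat from TDRoRInstance and runs it through IncreaseStat with ChangeInStat.
; The result goes to the player pawn via SetHealth, SetDamage or AddFireRate.
; It then debug-prints the stat and Rarity, which is only used for that print here, and destroys itself.
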(event `self.StaticMesh.OnComponentBeginOverlap`
  (params (OverlappedComponent :type "PrimitiveComponent Object Reference") (OtherActor :type "Actor Object Reference") (OtherComp :type "PrimitiveComponent Object Reference") (OtherBodyIndex :type Integer) (bFromSweep :type Boolean) (SweepResult :type "HitResult Structure (by ref)"))
  (cast `/Game/TwinStickBP/Blueprints/TwinStickPawn` OtherActor)
  (bind _astdro_rinstance (cast `/Game/TDRoR/GameManagers/TDRoRInstance` (`GameplayStatics.GetGameInstance`)))
  (bind _returnvalue (`self.IncreaseStat` (select `statToInrease` (`self.stat`) :`Health` (`/Game/TDRoR/GameManagers/TDRoRInstance.currentPlayerHealth` _astdro_rinstance) :`Damage` (`/Game/TDRoR/GameManagers/TDRoRInstance.currentPlayerDamage` _astdro_rinstance) :`FireRate` (`/Game/TDRoR/GameManagers/TDRoRInstance.currentPlayerFireRate` _astdro_rinstance)) (`self.changeInStat`)))
  (bind _astwin_stick_pawn (cast `/Game/TwinStickBP/Blueprints/TwinStickPawn` (`GameplayStatics.GetPlayerPawn` 0)))
  (if (select `statToInrease` (`self.stat`) :`Health` true)
    (`/Game/TwinStickBP/Blueprints/TwinStickPawn.Set Health` _astwin_stick_pawn _returnvalue)
    ;[1 1 1] Debugging
    (`KismetSystemLibrary.PrintString` (select `statToInrease` (`self.stat`) :`Health` "Health :" :`Damage` "Damage :" :`FireRate` "Fire Rate :") :!label _label)
    (`KismetSystemLibrary.PrintString` (`KismetStringLibrary.Conv_DoubleToString` _returnvalue))
    (`KismetSystemLibrary.PrintString` "Rarity")
    (`KismetSystemLibrary.PrintString` (select `itemRatiry` (`self.rarity`) :`Common` "Common" :`Uncommon` "Uncomon" :`Rare` "Rare" :`Mythic` "Mythic"))
    (`self.K2_DestroyActor`)
    (elif (select `statToInrease` (`self.stat`) :`Damage` true)
      (`/Game/TwinStickBP/Blueprints/TwinStickPawn.Set Damage` _astwin_stick_pawn _returnvalue)
      (goto _label)
      (elif (select `statToInrease` (`self.stat`) :`FireRate` true)
        (`/Game/TwinStickBP/Blueprints/TwinStickPawn.Add Fire Rate` _astwin_stick_pawn _returnvalue)
        (goto _label)))))

(fn `UserConstructionScript`)