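; Base melee enemy that bites the player on trigger overlap and rewards experience and currency on death.
; Health and damage scale from a monster stat card and CurrentLevel at BeginPlay; spawn cost also scales with level.
; A GameInstance three-minute event increments the level without recomputing health or damage.
; Attack only toggles a timed flag, which the bite ignores; death also spawns money pickups before destroying the actor.
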(event `self.ReceiveTick`
  (params (DeltaSeconds :type "Float (single-precision)")))

(event `self.ReceiveBeginPlay`
  (set `self.AIControllerRef` (`AIBlueprintHelperLibrary.GetAIController` self))
  (`self.SetupStats`)
  (bind _astdro_rinstance (cast `/Game/TDRoR/Blueprints/GameManagers/TDRoRInstance` (`GameplayStatics.GetGameInstance`)))
  (bind _output_get (set `self.GameInstance` _astdro_rinstance))
  (add `/Game/TDRoR/Blueprints/GameManagers/TDRoRInstance.3Minutemark` _output_get (delegate `Increase Level On 3 Minute Interval`)))

(event `Increase Level On 3 Minute Interval`
  (`/Engine/EditorBlueprintResources/StandardMacros.IncrementInt` (`self.CurrentLevel`)
    (:`  `
      (`KismetSystemLibrary.PrintString` (`KismetStringLibrary.Concat_StrStr` (`KismetSystemLibrary.GetObjectName` self) " |  New Level :" (`KismetStringLibrary.Conv_IntToString` (`self.CurrentLevel`)))))))

(event `self.ReceiveAnyDamage`
  (params (Damage :type "Float (single-precision)") (DamageType :type "DamageType Object Reference") (InstigatedBy :type "Controller Object Reference") (DamageCauser :type "Actor Object Reference"))
  (set `self.currentHealth` (- (`self.currentHealth`) Damage))
  (`self.Check Health`))

(event `Attack`
  (set `self.IsAttacking` true)
  (`KismetSystemLibrary.Delay` (`self.AttackTimer`))
  (set `self.IsAttacking` false))

(event `self.Bite_Attack_Trigger.OnComponentBeginOverlap`
  (params (OverlappedComponent :type "PrimitiveComponent Object Reference") (OtherActor :type "Actor Object Reference") (OtherComp :type "PrimitiveComponent Object Reference") (OtherBodyIndex :type Integer) (bFromSweep :type Boolean) (SweepResult :type "HitResult Structure (by ref)"))
  (bind _asdrongo_player_character (cast `/Game/TDRoR/Characters/Heroes/Drongo/DrongoPlayerCharacter` OtherActor))
  (`GameplayStatics.ApplyDamage` _asdrongo_player_character (`KismetMathLibrary.Conv_IntToDouble` (`self.MeleeDamage`)) null self))

(fn `Check Health`
  (bind _returnvalue (`GameplayStatics.GetGameInstance`))
  (if (<= (`self.currentHealth`) 0.0)
    (set `self.isDead` true)
    (bind _astdro_rinstance (cast `/Game/TDRoR/Blueprints/GameManagers/TDRoRInstance` _returnvalue))
    (`/Game/TDRoR/Blueprints/GameManagers/TDRoRInstance.AddToExp` _astdro_rinstance (`self.expGivenOnDeath`))
    (message `/Game/TDRoR/Blueprints/GameManagers/BPI_Interact.Gain Currency Event` _returnvalue (`self.currencyGivenOnDeath`))
    (`self.SpawnPointEffect` 5)
    (`self.K2_DestroyActor`)))

(fn `GetCost`
  (returns (`Spawn Cost` :type "Float (double-precision)"))
  (return (* (`self.CurrentLevel`) (`Monster_StatCard.baseSpawnCost` (`self.Monster_StatCard`)))))

(fn `GetMonsterStatCard`
  (returns (Monster_StatCard :type "Monster_StatCard Object Reference"))
  (return (`self.Monster_StatCard`)))

(fn `OnInteract`
  (returns (Success :type Boolean))
  (return false))

(fn `SetupStats`
  (bind _monster_statcard (`self.Monster_StatCard`))
  (set `self.MeleeDamage` (`KismetMathLibrary.Round` (+ (`Monster_StatCard.baseDamage` _monster_statcard) (* (`self.CurrentLevel`) (`Monster_StatCard.damagePerLevel` _monster_statcard)))))
  (bind _output_get (set `self.MaxHealth` (`KismetMathLibrary.Conv_IntToDouble` (`KismetMathLibrary.Round` (+ (`Monster_StatCard.baseHealth` _monster_statcard) (* (`self.CurrentLevel`) (`Monster_StatCard.healthPerLevel` _monster_statcard)))))))
  (set `self.currentHealth` _output_get)
  (`KismetSystemLibrary.PrintString` (`KismetStringLibrary.Concat_StrStr` (`KismetSystemLibrary.GetObjectName` self) " : " "Health : " (`KismetStringLibrary.Conv_DoubleToString` (`self.MaxHealth`)) " | " "Damage : " (`KismetStringLibrary.Conv_IntToString` (`self.MeleeDamage`)))))

(fn `SpawnPointEffect`
  (params (SpawnForEvery :type Integer :default 5))
  (for _ (range (+ (/ (`self.currencyGivenOnDeath`) SpawnForEvery) 1))
    (`|SpawnActorFromClass` "/Game/TDRoR/Blueprints/CollectableEffect/Collectable_Base_Money.Collectable_Base_Money_C" (`KismetMathLibrary.MakeTransform` (`self.K2_GetActorLocation`)) "AlwaysSpawn" "OverrideRootScale" null null null)))

(fn `UserConstructionScript`)