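; Great spider boss enemy with claw attacks and health-based phases, notifying the game mode when destroyed.
; Attack and ComboAttackSave drive a buffered combo toggling claw components, whose overlaps damage the player while attacking; the counter jumps from 0 to 2, skipping the right-claw step.
; Damage updates BossState, raising walk speed once each at three-quarter and half health; the half-health check overwrites IsDead.
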(event `self.ReceiveBeginPlay`
  (`parent.ReceiveBeginPlay`)
  (set `self.AttackTimer` 2.467)
  (`ActorComponent.SetActive` (`self.LeftClaw`) false false)
  (`ActorComponent.SetActive` (`self.RightClaw`) false false))

(event `self.ReceiveTick`
  (params (DeltaSeconds :type "Float (single-precision)"))
  (`parent.ReceiveTick` DeltaSeconds))

(event `self.ReceiveDestroyed`
  (`parent.ReceiveDestroyed`)
  (bind _astdro_rgame_mode (cast `/Game/TDRoR/Blueprints/GameManagers/TDRoRGameMode` (`GameplayStatics.GetGameMode`)))
  (`/Game/TDRoR/Blueprints/GameManagers/TDRoRGameMode.OnBossFinish` _astdro_rgame_mode))

(event `self.ReceiveAnyDamage`
  (params (Damage :type "Float (single-precision)") (DamageType :type "DamageType Object Reference") (InstigatedBy :type "Controller Object Reference") (DamageCauser :type "Actor Object Reference"))
  (`parent.ReceiveAnyDamage` Damage null null null)
  (`self.BossState_Health`)
  (`self.CheckCurrentState`))

(event `self.Attack`
  (if (`self.IsAttacking`)
    (set `self.SaveAttack` true)
    (else
      (set `self.IsAttacking` true)
      (switch `int` (`self.AttackCount`) :!label _label
        (:`0`
          (set `self.AttackCount` 2)
          (`ActorComponent.SetActive` (`self.LeftClaw`) true false))
        (:`1`
          (set `self.AttackCount` 1)
          (`ActorComponent.SetActive` (`self.LeftClaw`) false false)
          (`ActorComponent.SetActive` (`self.RightClaw`) true false))
        (:`2`
          (set `self.AttackCount` 0)
          (`self.ResetCombo`))))))

(event `ComboAttackSave`
  (if (`self.SaveAttack`)
    (set `self.SaveAttack` false)
    (goto _label)))

(event `ResetCombo`
  (set `self.AttackCount` 0)
  (set `self.SaveAttack` false)
  (set `self.IsAttacking` false)
  (`ActorComponent.SetActive` (`self.LeftClaw`) false false)
  (`ActorComponent.SetActive` (`self.RightClaw`) false false))

(event `self.RightClaw.OnComponentBeginOverlap`
  (params (OverlappedComponent :type "PrimitiveComponent Object Reference") (OtherActor :type "Actor Object Reference") (OtherComp :type "PrimitiveComponent Object Reference") (OtherBodyIndex :type Integer) (bFromSweep :type Boolean) (SweepResult :type "HitResult Structure (by ref)"))
  (bind (_asdrongo_player_character _bsuccess) (cast `/Game/TDRoR/Characters/Heroes/Drongo/DrongoPlayerCharacter` OtherActor :!pure true))
  (if _bsuccess
    (if (`self.IsAttacking`)
      (`GameplayStatics.ApplyDamage` _asdrongo_player_character 10.0 null self))))

(event `self.LeftClaw.OnComponentBeginOverlap`
  (params (OverlappedComponent :type "PrimitiveComponent Object Reference") (OtherActor :type "Actor Object Reference") (OtherComp :type "PrimitiveComponent Object Reference") (OtherBodyIndex :type Integer) (bFromSweep :type Boolean) (SweepResult :type "HitResult Structure (by ref)"))
  (bind (_asdrongo_player_character _bsuccess) (cast `/Game/TDRoR/Characters/Heroes/Drongo/DrongoPlayerCharacter` OtherActor :!pure true))
  (if _bsuccess
    (if (`self.IsAttacking`)
      (`GameplayStatics.ApplyDamage` _asdrongo_player_character 10.0 null self))))

(fn `BossState_Health`
  (`|ExecutionSequence`
    (:`then_0`
      (if (<= (`self.Health`) 0.0)
        (set `self.BossState` "NewEnumerator4")))
    (:`then_1`
      (if (<= (`self.Health`) (/ (`self.MaxHealth`) 2.0))
        (set `self.BossState` "NewEnumerator2")))
    (:`then_2`
      (if (and (<= (`self.Health`) (- (`self.MaxHealth`) (/ (`self.MaxHealth`) 4.0))) (`|EnumInequality` (`self.BossState`) "NewEnumerator2"))
        (set `self.BossState` "NewEnumerator1")))
    (:`then_3`
      (if (and (>= (`self.Health`) (- (`self.MaxHealth`) (/ (`self.MaxHealth`) 4.0))) (or (`|EnumInequality` (`self.BossState`) "NewEnumerator1") (`|EnumInequality` (`self.BossState`) "NewEnumerator2")))
        (set `self.BossState` "NewEnumerator0")))))

(fn `CheckCurrentState`
  (switch `/Game/TDRoR/Enemies/Enemy_Great_Spider/BossState` (`self.BossState`)
    (:`NewEnumerator0`
      (if (not (`self.isSpawnedTrigger`))
        (set `self.isSpawnedTrigger` true)))
    (:`NewEnumerator1`
      (`self.ThreeQtrHealthSetup`))
    (:`NewEnumerator2`
      (`self.HalfHealthStatsSetup`))))

(fn `HalfHealthStatsSetup`
  (bind _charactermovement (`self.CharacterMovement`))
  (if (not (`self.isAtHalfTriggered`))
    (set `CharacterMovementComponent.MaxWalkSpeed` (+ (`MovementComponent.GetMaxSpeed` _charactermovement) (`self.MoveSpeedIncrease`)) _charactermovement)
    (set `self.isAtHalfTriggered` true)))

(fn `ThreeQtrHealthSetup`
  (bind _charactermovement (`self.CharacterMovement`))
  (if (not (`self.isThreeQtrTriggered`))
    (set `CharacterMovementComponent.MaxWalkSpeed` (+ (`MovementComponent.GetMaxSpeed` _charactermovement) (`self.MoveSpeedIncrease`)) _charactermovement)
    (set `self.isThreeQtrTriggered` true)))

(fn `UserConstructionScript`
  (`parent.UserConstructionScript`))