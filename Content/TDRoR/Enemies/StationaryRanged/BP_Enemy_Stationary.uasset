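; BP_Enemy_Stationary is a ranged enemy that shoots at the player and optionally pursues them.
; PawnSensing sight turns it toward the player, fires basic projectiles on a delay-gated cooldown, and calls AIMoveTo unless Stationary is set.
; Hearing shares the facing logic but reads the sight-cast player reference.
; Health scales with the game instance's current stage, drops with damage, and Tick destroys the actor at zero.
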(event `self.PawnSensing.OnHearNoise`
  (params (Instigator :type "Pawn Object Reference") (Location :type "Vector Structure (by ref)") (Volume :type "Float (single-precision)"))
  (bind _asdrongo_player_character (cast `/Game/TDRoR/Characters/Heroes/Drongo/DrongoPlayerCharacter` Instigator))
  (set `self.PlayerDetected` _asdrongo_player_character)
  ;[1 1 1] Face Player
  (`self.K2_SetActorRotation` (`KismetMathLibrary.FindLookAtRotation` (`self.K2_GetActorLocation`) (`self.K2_GetActorLocation` (stale `self.PawnSensing.OnSeePawn` _asdrongo_player_character))) :!label _label))

(event `self.PawnSensing.OnSeePawn`
  (params (Pawn :type "Pawn Object Reference"))
  (bind _playerdetected (`self.PlayerDetected`))
  (bind _asdrongo_player_character (cast `/Game/TDRoR/Characters/Heroes/Drongo/DrongoPlayerCharacter` Pawn))
  (set `self.PlayerDetected` _asdrongo_player_character)
  (`|ExecutionSequence`
    (:`then_0`
      (goto _label))
    (:`then_1`
      ;[1 1 1] Shoot at player on Timer
      (if (`self.SpawnProjectile`)
        (`|SpawnActorFromClass` "/Game/TDRoR/Projectiles/Enemy_Projectile_Basic.Enemy_Projectile_Basic_C" (`SceneComponent.K2_GetComponentToWorld` (`self.ProjSpawnLoc`)) "Undefined" "OverrideRootScale" null null)
        (set `self.SpawnProjectile` false)
        (`KismetSystemLibrary.Delay` 1.5)
        (set `self.SpawnProjectile` true)))
    (:`then_2`
      ;[0.1823 0 0] Note: I want the enemy to not move while shooting, then resume moving
      (if (not (`self.Stationary`))
        ;[1 1 1] Move towards the player
        (`|AIMoveTo` self (`SceneComponent.K2_GetComponentLocation` (`Character.Mesh` _playerdetected)) _playerdetected 5.0 true)))))

(event `self.ReceiveAnyDamage`
  (params (Damage :type "Float (single-precision)") (DamageType :type "DamageType Object Reference") (InstigatedBy :type "Controller Object Reference") (DamageCauser :type "Actor Object Reference"))
  (`self.RemoveHealth` Damage)
  (`KismetSystemLibrary.PrintString` (`KismetStringLibrary.Conv_DoubleToString` (`self.Health`))))

(event `self.ReceiveTick`
  (params (DeltaSeconds :type "Float (single-precision)"))
  (if (<= (`self.Health`) 0.0)
    (`self.K2_DestroyActor`)))

(event `self.ReceiveBeginPlay`
  (bind _astdro_rinstance (cast `/Game/TDRoR/Blueprints/GameManagers/TDRoRInstance` (`GameplayStatics.GetGameInstance`)))
  (set `self.Health` (* (`/Game/TDRoR/Blueprints/GameManagers/TDRoRInstance.currentStage` _astdro_rinstance) (`self.Health`))))

(fn `RemoveHealth`
  (params (`Health Removed` :type "Float (double-precision)"))
  (set `self.Health` (- (`self.Health`) `Health Removed`)))

(fn `UserConstructionScript`)