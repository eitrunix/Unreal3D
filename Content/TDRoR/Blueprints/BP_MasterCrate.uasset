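; BP_MasterCrate is a lootable container, either a cash box that grants currency or a tiered crate that costs currency, with type-colored materials and random yaw.
; Box overlap shows the player an interact prompt or cost; CheckLooted calls C++ LootCrate's Loot, opens doors and drawer, and messages the game instance.
; BeginPlay and Tick both multiply the stored base cost or money by CurrentStage, so values compound.
; The construction script forces Type to CashBox.
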(event `self.ReceiveBeginPlay`
  (if (`|EnumEquality` (`self.type`) "CashBox") :!label _label
    (`self.CalcMoneyInChest`)
    (else
      (`self.CalcCost`))))

(event `self.ReceiveTick`
  (params (DeltaSeconds :type "Float (single-precision)"))
  (goto _label))

(event `CheckLooted`
  (bind _returnvalue (`GameplayStatics.GetGameInstance`))
  (bind _tmpcurrency (`self.tmpCurrency`))
  ;[1 1 1] Check if looted already, if not loot box
  (if (not (`self.givenLoot`))
    ;[1 1 1] Looting Function
    ;;[1 1 1] From LootCrate.cpp
    (bind _returnvalue_2 (`self.Loot`))
    (set `self.tmpCurrency` _returnvalue_2)
    (`self.OpenContainer`)
    (if (`|EnumEquality` (`self.type`) "CashBox")
      (message `/Game/TDRoR/GameManagers/BPI_Interact.Gain Currency Event` _returnvalue _tmpcurrency)
      (else
        (message `/Game/TDRoR/GameManagers/BPI_Interact.Take Currency Event` _returnvalue _tmpcurrency)))))

(event `self.Box.OnComponentBeginOverlap`
  (params (OverlappedComponent :type "PrimitiveComponent Object Reference") (OtherActor :type "Actor Object Reference") (OtherComp :type "PrimitiveComponent Object Reference") (OtherBodyIndex :type Integer) (bFromSweep :type Boolean) (SweepResult :type "HitResult Structure (by ref)"))
  (bind _widget (`self.Widget`))
  (bind _asw_pick_up_widget (cast `/Game/TDRoR/Widgets/W_PickUpWidget` (`WidgetComponent.GetUserWidgetObject` _widget) :!pure true))
  ;[1 1 1] Interact Widget
  (cast `/Game/TDRoR/Blueprints/DrongoPlayerCharacter` OtherActor)
  (if (not (`self.opened`))
    (set `self.inOpenRange` true)
    (if (`|EnumEquality` (`self.type`) "CashBox")
      (`/Game/TDRoR/Widgets/W_PickUpWidget.Set_CrateText` _asw_pick_up_widget "Press \"F\" to Interact")
      (else
        (`/Game/TDRoR/Widgets/W_PickUpWidget.Set_CrateText` _asw_pick_up_widget (`self.TmpCost`))))
    (`SceneComponent.SetVisibility` _widget true false)))

(event `self.Box.OnComponentEndOverlap`
  (params (OverlappedComponent :type "PrimitiveComponent Object Reference") (OtherActor :type "Actor Object Reference") (OtherComp :type "PrimitiveComponent Object Reference") (OtherBodyIndex :type Integer))
  ;[1 1 1] Interact Widget
  (cast `/Game/TDRoR/Blueprints/DrongoPlayerCharacter` OtherActor)
  (set `self.inOpenRange` false)
  (`SceneComponent.SetVisibility` (`self.Widget`) false false))

(event `CalcCost`
  (bind _astdro_rinstance (cast `/Game/TDRoR/GameManagers/TDRoRInstance` (`GameplayStatics.GetGameInstance`)))
  (bind _output_get (set `self.baseChestCost` (* (`self.baseChestCost`) (`/Game/TDRoR/GameManagers/TDRoRInstance.currentStage` _astdro_rinstance))))
  (set `self.TmpCost` (`KismetTextLibrary.Conv_IntToText` _output_get)))

(event `CalcMoneyInChest`
  (bind _astdro_rinstance (cast `/Game/TDRoR/GameManagers/TDRoRInstance` (`GameplayStatics.GetGameInstance`)))
  (set `self.baseMoneyInChest` (* (`/Game/TDRoR/GameManagers/TDRoRInstance.currentStage` _astdro_rinstance) (`self.baseMoneyInChest`))))

(fn `OpenContainer`
  ;[1 1 1] Movement
  (`SceneComponent.K2_SetRelativeRotation` (`self.Locker05Door01`) (`KismetMathLibrary.MakeRotator` 0.0 0.0 (`self.Door01Rotation`)) false false)
  (`SceneComponent.K2_SetRelativeRotation` (`self.Locker05Door02`) (`KismetMathLibrary.MakeRotator` 0.0 0.0 (* (`self.Door02Rotation`) -1.0)) false false)
  (`SceneComponent.K2_AddRelativeLocation` (`self.Table05Drawer01`) (`KismetMathLibrary.MakeVector` 0.0 (* (`self.Drawer01Position`) -1.0)) false false))

(fn `RandomRotation`
  (bind _box (`self.Box`))
  (bind (_returnvalue_roll _returnvalue_pitch) (`KismetMathLibrary.BreakRotator` (`SceneComponent.K2_GetComponentRotation` _box)))
  (`SceneComponent.K2_SetRelativeRotation` _box (`KismetMathLibrary.MakeRotator` _returnvalue_roll _returnvalue_pitch (`KismetMathLibrary.RandomFloatInRange` -360.0 360.0)) false false))

(fn `SetMesh`
  (`PrimitiveComponent.SetMaterial` (`self.Locker05Door01`) 0 (select `CrateType` (`self.type`) :`CashBox` "/Game/Geometry/ScienceLab/Materials/Furniture/MI_FurnitureB.MI_FurnitureB" :`Small` "/Game/Geometry/ScienceLab/Materials/Furniture/MI_Furniture_Blue.MI_Furniture_Blue" :`Medium` "/Game/Geometry/ScienceLab/Materials/Furniture/MI_Furniture_Green.MI_Furniture_Green" :`Large` "/Game/Geometry/ScienceLab/Materials/Furniture/MI_Furniture_Red.MI_Furniture_Red" :!type "MaterialInterface Object Reference"))
  (`PrimitiveComponent.SetMaterial` (`self.Table05Drawer01`) 0 (select `CrateType` (`self.type`) :`CashBox` "/Game/Geometry/ScienceLab/Materials/Furniture/MI_FurnitureB.MI_FurnitureB" :`Small` "/Game/Geometry/ScienceLab/Materials/Furniture/MI_Furniture_Blue.MI_Furniture_Blue" :`Medium` "/Game/Geometry/ScienceLab/Materials/Furniture/MI_Furniture_Green.MI_Furniture_Green" :`Large` "/Game/Geometry/ScienceLab/Materials/Furniture/MI_Furniture_Red.MI_Furniture_Red" :!type "MaterialInterface Object Reference"))
  (`PrimitiveComponent.SetMaterial` (`self.Locker05Door02`) 0 (select `CrateType` (`self.type`) :`CashBox` "/Game/Geometry/ScienceLab/Materials/Furniture/MI_FurnitureB.MI_FurnitureB" :`Small` "/Game/Geometry/ScienceLab/Materials/Furniture/MI_Furniture_Blue.MI_Furniture_Blue" :`Medium` "/Game/Geometry/ScienceLab/Materials/Furniture/MI_Furniture_Green.MI_Furniture_Green" :`Large` "/Game/Geometry/ScienceLab/Materials/Furniture/MI_Furniture_Red.MI_Furniture_Red" :!type "MaterialInterface Object Reference"))
  (`PrimitiveComponent.SetMaterial` (`self.Locker05`) 0 (select `CrateType` (`self.type`) :`CashBox` "/Game/Geometry/ScienceLab/Materials/Furniture/MI_FurnitureB.MI_FurnitureB" :`Small` "/Game/Geometry/ScienceLab/Materials/Furniture/MI_Furniture_Blue.MI_Furniture_Blue" :`Medium` "/Game/Geometry/ScienceLab/Materials/Furniture/MI_Furniture_Green.MI_Furniture_Green" :`Large` "/Game/Geometry/ScienceLab/Materials/Furniture/MI_Furniture_Red.MI_Furniture_Red" :!type "MaterialInterface Object Reference")))

(fn `UserConstructionScript`
  (set `self.type` "CashBox")
  (`SceneComponent.SetVisibility` (`self.Widget`) false false)
  (`self.SetMesh`)
  (`self.RandomRotation`))