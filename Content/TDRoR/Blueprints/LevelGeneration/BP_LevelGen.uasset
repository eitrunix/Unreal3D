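; Procedural level generator that builds a seeded, tile-grid map of rooms and corridors from its construction script.
; Rooms are randomly sized, optionally culled with a flood fill keeping connected tiles, and placed in one of eight directions from the previous or a branched room.
; Straight corridors join consecutive rooms whose sides overlap with a gap between them.
; SpawnTiles adds floor instances and walls on edges lacking a neighbouring tile.
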(event `Generate Map`
  (`KismetSystemLibrary.FlushPersistentDebugLines`)
  (for _index (range (`self.RoomCount`))
    ;[1 1 1] Generate First Room at (0,0,0) Relative
    (if (== _index 0)
      (bind (_floortiles _location_ _extents) (`self.MakeFloorArea` (`self.PrevLocation`)))
      (set `self.FloorTiles` _floortiles)
      (`BlueprintMapLibrary.Map_Add` (`self.Rooms`) _location_ _extents)
      (elif (`self.Branching`)
        (bind _keys (`BlueprintMapLibrary.Map_Keys` (`self.Rooms`)))
        (if (and (>= (`KismetArrayLibrary.Array_LastIndex` _keys) (+ (`self.BranchingThreshold`) (`self.LastBranch`))) (`KismetMathLibrary.RandomBoolWithWeightFromStream` (`self.BranchChance`) (`self.Stream`)))
          ;[1 1 1] Get Previous Room to Branch From
          (bind _keys_2 (`BlueprintMapLibrary.Map_Keys` (`self.Rooms`) :!label _label))
          (bind _returnvalue (`KismetArrayLibrary.Array_LastIndex` _keys_2))
          (set `self.PrevLocation` (`|GetArrayItem` _keys_2 (`KismetMathLibrary.RandomIntegerFromStream` _returnvalue (`self.Stream`))))
          (set `self.LastBranch` _returnvalue)
          ;[1 1 1] Find Location to Place Next Room, Calc floor time for new room
          (bind (_valid _new_location) (`self.Room_FindNextLocation` :!label _label_2))
          (if _valid
            (bind _output_get (set `self.NextLocation` _new_location))
            (bind (_floortiles_2 _location__2 _extents_2) (`self.MakeFloorArea` _output_get))
            (`KismetArrayLibrary.Array_Append` (`self.FloorTiles`) _floortiles_2)
            (`BlueprintMapLibrary.Map_Add` (`self.Rooms`) _location__2 _extents_2)
            ;[1 1 1] Make Corridor between last two rooms
            (bind _corridor_tiles (`self.Corridors_MapCorridors` (`self.PrevLocation`) (`self.NextLocation`)))
            (`KismetArrayLibrary.Array_Append` (`self.CorridorTiles`) _corridor_tiles)
            ;[1 1 1] Update Location for next Loop
            (set `self.PrevLocation` (`self.NextLocation`))
            (else
              (goto _label))))
        (else
          (goto _label_2)))))
  (`self.SpawnTiles`))

(fn `Corridor_Make_x`
  (params (From :type "IntVector Structure") (To :type "IntVector Structure"))
  (returns (FloorTiles :type "Array of IntVector Structure"))
  (locals (Tiles :type "Array of IntVector Structure"))
  (bind (_x _y _z) (break `IntVector` From))
  (for _index (range (`KismetMathLibrary.Abs_Int` (- (`.X` (break `IntVector` From)) (`.X` (break `IntVector` To)))))
    (`KismetArrayLibrary.Array_Add` (`local.Tiles`) (make `IntVector` (+ _x _index) _y _z)))
  (return (`local.Tiles`)))

(fn `Corridor_Make_Y`
  (params (From :type "IntVector Structure") (To :type "IntVector Structure"))
  (returns (FloorTiles :type "Array of IntVector Structure"))
  (locals (Tiles :type "Array of IntVector Structure"))
  (bind (_x _y _z) (break `IntVector` From))
  (for _index (range (`KismetMathLibrary.Abs_Int` (- (`.Y` (break `IntVector` From)) (`.Y` (break `IntVector` To)))))
    (`KismetArrayLibrary.Array_Add` (`local.Tiles`) (make `IntVector` _x (+ _y _index) _z)))
  (return (`local.Tiles`)))

(fn `Corridors_MapCorridors`
  (params (`Room A` :type "IntVector Structure") (`Room B` :type "IntVector Structure"))
  (returns (`Corridor Tiles` :type "Array of IntVector Structure"))
  (locals (AX :type Integer) (AY :type Integer) (AZ :type Integer) (AX2 :type Integer) (AY2 :type Integer) (BX :type Integer) (BY :type Integer) (BZ :type Integer) (BX2 :type Integer) (BY2 :type Integer) (`Out X` :type Integer :default 0) (PointA :type "IntVector Structure") (PointB :type "IntVector Structure") (`Out Y` :type Integer :default 0) (Tiles :type "Array of IntVector Structure"))
  (bind (_x _y _z) (break `IntVector` `Room A`))
  (bind (_x_2 _y_2 _z_2) (break `IntVector` `Room B`))
  (bind _rooms (`self.Rooms`))
  (bind (_x_3 _y_3) (break `IntVector` (`BlueprintMapLibrary.Map_Find` _rooms `Room A`)))
  (bind (_x_4 _y_4) (break `IntVector` (`BlueprintMapLibrary.Map_Find` _rooms `Room B`)))
  (bind _returnvalue (`KismetMathLibrary.RandomIntegerInRangeFromStream` (`KismetMathLibrary.Max` (`local.AX`) (`local.BX`)) (`KismetMathLibrary.Min` (`local.AX2`) (`local.BX2`)) (`self.Stream`)))
  (bind _returnvalue_2 (`KismetMathLibrary.RandomIntegerInRangeFromStream` (`KismetMathLibrary.Max` (`local.AY`) (`local.BY`)) (`KismetMathLibrary.Min` (`local.AY2`) (`local.BY2`)) (`self.Stream`)))
  (`self.LevelGen_Debug` `Room A` `Room B`)
  (set `local.AX` _x)
  (set `local.AY` _y)
  (set `local.AZ` _z)
  (set `local.AX2` _x_3)
  (set `local.AY2` _y_3)
  (set `local.BX` _x_2)
  (set `local.BY` _y_2)
  (set `local.BZ` _z_2)
  (set `local.BX2` _x_4)
  (set `local.BY2` _y_4)
  (`|ExecutionSequence`
    (:`then_0`
      ;[1 1 1] Are Rooms Parallel on X with overlapping sides
      (if (<= (`KismetMathLibrary.Max` (`local.AX`) (`local.BX`)) (`KismetMathLibrary.Min` (`local.AX2`) (`local.BX2`)))
        ;[1 1 1] Room B to the Right?
        (if (> (`local.BY`) (`local.AY`))
          ;[1 1 1] Rooms Not Merged?
          (if (> (- (`local.BY`) (`local.AY2`)) 1)
            ;[1 1 1] Make Corridor from A to B on Y Axis
            (bind _output_get (set `local.Out X` _returnvalue))
            (set `local.PointA` (make `IntVector` _output_get (`local.AY2`) (`local.AZ`)))
            (set `local.PointB` (make `IntVector` _output_get (`local.BY`) (`local.BZ`)))
            (bind _floortiles (`self.Corridor_Make_Y` (`local.PointA`) (`local.PointB`)))
            (set `local.Tiles` _floortiles))
          (else
            ;[1 1 1] Rooms Not Merged?
            (if (> (- (`local.AY`) (`local.BY2`)) 1)
              ;[1 1 1] Make Corridor from B to A on Y Axis
              (bind _output_get_2 (set `local.Out X` _returnvalue))
              (set `local.PointA` (make `IntVector` _output_get_2 (`local.AY`) (`local.AZ`)))
              (set `local.PointB` (make `IntVector` _output_get_2 (`local.BY2`) (`local.BZ`)))
              (bind _floortiles_2 (`self.Corridor_Make_Y` (`local.PointB`) (`local.PointA`)))
              (set `local.Tiles` _floortiles_2))))
        (else
          ;[1 1 1] Are Rooms Parallel on Y with overlapping sides
          (if (<= (`KismetMathLibrary.Max` (`local.AY`) (`local.BY`)) (`KismetMathLibrary.Min` (`local.AY2`) (`local.BY2`)))
            ;[1 1 1] Room B in Front?
            (if (> (`local.BX`) (`local.AX`))
              ;[1 1 1] Rooms Not Merged?
              (if (> (- (`local.BX`) (`local.AX2`)) 1)
                ;[1 1 1] Make Corridor from A to B on X Axis
                (bind _output_get_3 (set `local.Out Y` _returnvalue_2))
                (set `local.PointA` (make `IntVector` (`local.AX2`) _output_get_3 (`local.AZ`)))
                (set `local.PointB` (make `IntVector` (`local.BX`) _output_get_3 (`local.BZ`)))
                (bind _floortiles_3 (`self.Corridor_Make_x` (`local.PointA`) (`local.PointB`)))
                (set `local.Tiles` _floortiles_3))
              (else
                ;[1 1 1] Rooms Not Merged?
                (if (> (- (`local.AX`) (`local.BX2`)) 1)
                  ;[1 1 1] Make Corridor from B to A on X Axis
                  (bind _output_get_4 (set `local.Out Y` _returnvalue_2))
                  (set `local.PointA` (make `IntVector` (`local.AX`) _output_get_4 (`local.AZ`)))
                  (set `local.PointB` (make `IntVector` (`local.BX2`) _output_get_4 (`local.BZ`)))
                  (bind _floortiles_4 (`self.Corridor_Make_x` (`local.PointB`) (`local.PointA`)))
                  (set `local.Tiles` _floortiles_4))))))))
    (:`then_1`
      (return (`local.Tiles`)))))

(fn `LevelGen_Debug`
  (params (`Room A` :type "IntVector Structure") (`Room B` :type "IntVector Structure"))
  (`KismetSystemLibrary.DrawDebugBox` (* (`KismetMathLibrary.Conv_IntVectorToVector` `Room A`) (`self.Scale`)) (10.0 10.0 50.0) (struct :`R` 1.0 :`B` 0.047002 :`A` 1.0) (struct) 500.0 50.0)
  (`KismetSystemLibrary.DrawDebugBox` (* (`KismetMathLibrary.Conv_IntVectorToVector` `Room B`) (`self.Scale`)) (10.0 10.0 50.0) (struct :`G` 0.493055 :`B` 0.191522 :`A` 1.0) (struct) 500.0 50.0)
  (`KismetSystemLibrary.DrawDebugBox` (* (`KismetMathLibrary.Conv_IntVectorToVector` `Room B`) (`self.Scale`)) (10.0 10.0 50.0) (struct :`G` 0.059509 :`B` 1.0 :`A` 1.0) (struct) 500.0 50.0)
  (`KismetSystemLibrary.DrawDebugBox` (* (`KismetMathLibrary.Conv_IntVectorToVector` `Room A`) (`self.Scale`)) (10.0 10.0 50.0) (struct :`R` 1.0 :`G` 0.931999 :`A` 1.0) (struct) 500.0 50.0)
  (return))

(fn `MakeFloorArea`
  (params (Location :type "IntVector Structure"))
  (returns (FloorTiles :type "Array of IntVector Structure") (`Location ` :type "IntVector Structure") (Extents :type "IntVector Structure"))
  (locals (RootLocation :type "IntVector Structure") (Out_X :type Integer :default 0) (Out_Y :type Integer :default 0) (Working :type Boolean :default true) (Tiles :type "Array of IntVector Structure") (ConnectedTiles :type "Array of IntVector Structure") (Extents_X :type "Array of Integer") (Extents_Y :type "Array of Integer") (TilesCopy :type "Array of IntVector Structure") (TileFound :type Boolean :default true) (LoopCount :type Integer))
  (bind _roomsize_min (`self.RoomSize_Min`))
  (bind _roomsize_max (`self.RoomSize_Max`))
  (bind _tilescopy (`local.TilesCopy`))
  (bind _connectedtiles (`local.ConnectedTiles`))
  (bind _tilescopy_2 (`local.TilesCopy`))
  (bind _out_y (`local.Out_Y`))
  (bind _stream (`self.Stream`))
  (bind (_x _y _z) (break `IntVector` (`local.RootLocation`)))
  (set `local.RootLocation` Location)
  (set `local.Out_X` (`KismetMathLibrary.RandomIntegerInRangeFromStream` _roomsize_min _roomsize_max _stream))
  (set `local.Out_Y` (`KismetMathLibrary.RandomIntegerInRangeFromStream` _roomsize_min _roomsize_max _stream))
  (for _index (range (* (`local.Out_X`) (`local.Out_Y`)))
    (`KismetArrayLibrary.Array_Add` (`local.Tiles`) (make `IntVector` (+ (/ _index _out_y) _x) (+ (mod _index _out_y) _y) _z)))
  (if (`self.FloorCulling`)
    (while (`local.Working`)
      (if (<= (`local.LoopCount`) (`self.MaxLoops`))
        ;[1 1 1] Randomly Cull Tiles from floor
        (set `local.TilesCopy` (`local.Tiles`))
        (for _ (range (+ (`KismetMathLibrary.Clamp` (- (`KismetMathLibrary.RandomIntegerInRangeFromStream` (`self.FloorCull_Min`) (`self.FloorCull_Max`) (`self.Stream`)) 1) 0 (/ (`KismetArrayLibrary.Array_Length` (`local.TilesCopy`)) 4)) 1))
          (`KismetArrayLibrary.Array_Remove` _tilescopy (`KismetMathLibrary.RandomIntegerFromStream` (`KismetArrayLibrary.Array_LastIndex` _tilescopy) (`self.Stream`))))
        ;[1 1 1] Check Neighbours for Connected Tiles, if So add to Connected Array
        (`KismetArrayLibrary.Array_Clear` _connectedtiles)
        (`KismetArrayLibrary.Array_Add` _connectedtiles (`|GetArrayItem` (`local.TilesCopy`)))
        (while (`local.TileFound`)
          (set `local.TileFound` false)
          (for _array_element (`local.ConnectedTiles`)
            (for _index_2 (range 4)
              (bind (_location _isinarray) (`self.TestRelativeTileLocation` _array_element _tilescopy_2 1))
              (bind (_location_2 _isinarray_2) (`self.TestRelativeTileLocation` _array_element _tilescopy_2 0 1))
              (bind (_location_3 _isinarray_3) (`self.TestRelativeTileLocation` _array_element _tilescopy_2 -1))
              (bind (_location_4 _isinarray_4) (`self.TestRelativeTileLocation` _array_element _tilescopy_2 0 -1))
              (if (select `int` _index_2 :`0` _isinarray :`1` _isinarray_2 :`2` _isinarray_3 :`3` _isinarray_4)
                (bind _returnvalue (select `int` _index_2 :`0` _location :`1` _location_2 :`2` _location_3 :`3` _location_4))
                (`KismetArrayLibrary.Array_Add` (`local.ConnectedTiles`) _returnvalue)
                (`KismetArrayLibrary.Array_RemoveItem` (`local.TilesCopy`) _returnvalue)
                (set `local.TileFound` true)))))
        (if (> (`KismetArrayLibrary.Array_Length` (`local.ConnectedTiles`)) (* (`self.RoomSize_Min`) (`self.RoomSize_Min`)))
          (set `local.Working` false)
          (else
            (set `local.Working` true)
            (`/Engine/EditorBlueprintResources/StandardMacros.IncrementInt` (`local.LoopCount`))))
        (else
          ;[1 1 1] Fail Out Without Cilling
          (set `local.Working` true)
          (set `local.ConnectedTiles` (`local.Tiles`)))))
    (else
      ;[1 1 1] Get Outter Extent Of Room
      (set `local.ConnectedTiles` (`local.Tiles`))))
  (for _array_element_2 (`local.ConnectedTiles`)
    (bind (_x_2 _y_2) (break `IntVector` _array_element_2))
    (`KismetArrayLibrary.Array_Add` (`local.Extents_X`) _x_2)
    (`KismetArrayLibrary.Array_Add` (`local.Extents_Y`) _y_2))
  (return (`local.ConnectedTiles`) (`local.RootLocation`) (make `IntVector` (`.MaxValue` (`KismetMathLibrary.MaxOfIntArray` (`local.Extents_X`))) (`.MaxValue` (`KismetMathLibrary.MaxOfIntArray` (`local.Extents_Y`))))))

(fn `Room_FindNextLocation`
  (returns (Valid :type Boolean) (`New Location` :type "IntVector Structure"))
  (locals (Directions :type "Array of Integer") (Searching :type Boolean :default true) (TestIndex :type Integer) (isValid :type Boolean) (NewLocation :type "IntVector Structure"))
  (bind _floortiles (`self.FloorTiles`))
  (bind _testindex (`local.TestIndex`))
  (bind _roomsize_max (`self.RoomSize_Max`))
  (bind _returnvalue (`KismetArrayLibrary.Array_LastIndex` (`local.Directions`)))
  (bind _returnvalue_2 (select `bool` (`self.Merging`) :`false` (+ _roomsize_max 1) :`true` _roomsize_max))
  (bind _returnvalue_3 (* _returnvalue_2 -1))
  (bind (_location _isinarray) (`self.TestRelativeTileLocation` (`self.PrevLocation`) _floortiles _returnvalue_2))
  (bind (_location_2 _isinarray_2) (`self.TestRelativeTileLocation` (`self.PrevLocation`) _floortiles _returnvalue_2 _returnvalue_2))
  (bind (_location_3 _isinarray_3) (`self.TestRelativeTileLocation` (`self.PrevLocation`) _floortiles 0 _returnvalue_2))
  (bind (_location_4 _isinarray_4) (`self.TestRelativeTileLocation` (`self.PrevLocation`) _floortiles _returnvalue_2 _returnvalue_3))
  (bind (_location_5 _isinarray_5) (`self.TestRelativeTileLocation` (`self.PrevLocation`) _floortiles _returnvalue_3))
  (bind (_location_6 _isinarray_6) (`self.TestRelativeTileLocation` :`RefLocation` (`self.PrevLocation`) :`X` _returnvalue_3 :`Y` _returnvalue_3))
  (bind (_location_7 _isinarray_7) (`self.TestRelativeTileLocation` (`self.PrevLocation`) _floortiles 0 _returnvalue_3))
  (bind (_location_8 _isinarray_8) (`self.TestRelativeTileLocation` (`self.PrevLocation`) _floortiles _returnvalue_3 _returnvalue_2))
  (set `local.Directions` (`|MakeArray` 0 1 2 3 4 5 6 7))
  (while (`local.Searching`)
    (if (>= _returnvalue 0)
      (set `local.TestIndex` (`KismetMathLibrary.RandomIntegerFromStream` _returnvalue (`self.Stream`)))
      (if (select `int` _testindex :`0` _isinarray :`1` _isinarray_2 :`2` _isinarray_3 :`3` _isinarray_8 :`4` _isinarray_5 :`5` _isinarray_6 :`6` _isinarray_7 :`7` _isinarray_4)
        (`KismetArrayLibrary.Array_Remove` (`local.Directions`) (`local.TestIndex`))
        (set `local.Searching` true)
        (else
          (set `local.Searching` false)
          (set `local.isValid` true)
          (set `local.NewLocation` (select `int` _testindex :`0` _location :`1` _location_2 :`2` _location_3 :`3` _location_8 :`4` _location_5 :`5` _location_6 :`6` _location_7 :`7` _location_4))))
      (else
        ;[1 1 1] Flag Invalid
        (set `local.Searching` false)
        (set `local.isValid` false))))
  (return (`local.isValid`) (`local.NewLocation`)))

(fn `SpawnTiles`
  (locals (NewLocalVar_0 :type "Vector Structure" :default (0.0 0.0 0.0)))
  (bind _scale (`self.Scale`))
  (`KismetArrayLibrary.Array_Append` (`self.FloorTiles`) (`self.CorridorTiles`))
  (for _array_element (`self.FloorTiles`)
    (`|ExecutionSequence`
      (:`then_0`
        (`InstancedStaticMeshComponent.AddInstance` (`self.Floor`) (`KismetMathLibrary.MakeTransform` (* (`KismetMathLibrary.Conv_IntVectorToVector` _array_element) (`self.Scale`)))))
      (:`then_1`
        ;[1 1 1] Spawn Walls
        (for _index (range 4)
          (if (not (select `int` _index :`0` (`.IsInArray` (`self.TestRelativeTileLocation` _array_element (`self.FloorTiles`) 0 1)) :`1` (`.IsInArray` (`self.TestRelativeTileLocation` _array_element (`self.FloorTiles`) 1)) :`2` (`.IsInArray` (`self.TestRelativeTileLocation` _array_element (`self.FloorTiles`) 0 -1)) :`3` (`.IsInArray` (`self.TestRelativeTileLocation` _array_element (`self.FloorTiles`) -1))))
            (switch `int` _index
              (:`0`
                (bind (_returnvalue_x _returnvalue_y) (`KismetMathLibrary.BreakVector` (* (`KismetMathLibrary.Conv_IntVectorToVector` _array_element) _scale)))
                (set `local.NewLocalVar_0` (`KismetMathLibrary.MakeVector` _returnvalue_x _returnvalue_y)))
              (:`1`
                (set `local.NewLocalVar_0` (`KismetMathLibrary.MakeVector` _returnvalue_x _returnvalue_y)))
              (:`2`
                (bind _returnvalue (- _returnvalue_x _scale))
                (bind _returnvalue_2 (- _returnvalue_y _scale))
                (set `local.NewLocalVar_0` (`KismetMathLibrary.MakeVector` _returnvalue _returnvalue_2)))
              (:`3`
                (set `local.NewLocalVar_0` (`KismetMathLibrary.MakeVector` _returnvalue _returnvalue_2))))
            (`InstancedStaticMeshComponent.AddInstance` (`self.Wall`) (`KismetMathLibrary.MakeTransform` (`local.NewLocalVar_0`) (select `int` _index :`0` (struct) :`1` (struct :`Yaw` 90.0) :`2` (struct :`Yaw` 180.0) :`3` (struct :`Yaw` -90.0) :!type "Rotator Structure")))))))))

(fn `UserConstructionScript`
  (`|ExecutionSequence`
    (:`then_0`
      ;[1 1 1] New Seed = True, Get new Random Seed.
      (if (`self.NewSeed`)
        (set `self.NewSeed` false)
        (bind _output_get (set `self.Seed` (`KismetMathLibrary.RandomInteger` 900000)))
        (`KismetMathLibrary.SetRandomStreamSeed` (`self.Stream`) _output_get)))
    (:`then_1`
      ;[1 1 1] Update Stream with Seed. Manual
      (`KismetMathLibrary.SetRandomStreamSeed` (`self.Stream`) (`self.Seed`)))
    (:`then_2`
      (`self.Generate Map`))))