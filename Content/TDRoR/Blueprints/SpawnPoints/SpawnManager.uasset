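; Spawn manager that spends a growing token budget to spawn enemies at the level's BP_SpawnPoints.
; The game instance's start-timer event builds an enemy-to-cost map for the current environment from class defaults.
; Each 10-second timer event grows tokens by the instance's Coeff, then gives active spawners random enemies, rerolling unaffordable picks until tokens fall below a floor.
; Rare-environment setup is an empty stub, and its test roll is uncalled here.
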(event `self.ReceiveBeginPlay`
  (`self.GetAllSpawnPoints`)
  (`self.Calc Spawn Tokens`)
  (add `self.10SecondTimer` (delegate `AddSpawnPointToSpawn`))
  (add `self.RareEvironment` (delegate `RareEnvironmentSetup`))
  (bind _astdro_rinstance (cast `/Game/TDRoR/Blueprints/GameManagers/TDRoRInstance` (`GameplayStatics.GetGameInstance`)))
  (add `/Game/TDRoR/Blueprints/GameManagers/TDRoRInstance.StartTimer` _astdro_rinstance (delegate `Build Enemy List`)))

(event `Build Enemy List`
  (`self.BuildEnemyList`))

(event `AddSpawnPointToSpawn`
  (`self.Calc Spawn Tokens`)
  (`self.SpawnCheck`))

(event `RareEnvironmentSetup`)

(event `self.ReceiveTick`
  (params (DeltaSeconds :type "Float (single-precision)")))

(fn `BuildEnemyList`
  (locals (TmpClass :type "Actor Class Reference") (tmpIndex :type Integer))
  (bind _astdro_rinstance (cast `/Game/TDRoR/Blueprints/GameManagers/TDRoRInstance` (`GameplayStatics.GetGameInstance`)))
  (switch `/Game/TDRoR/Blueprints/LevelGeneration/EnvironmentEnum` (`/Game/TDRoR/Blueprints/GameManagers/TDRoRInstance.currentEnvironment` _astdro_rinstance)
    (:`NewEnumerator0`
      (for _array_element (`self.Enemies_Normal`)
        (bind _asenemy_base_class (castclass `/Game/TDRoR/Enemy/Enemy_Blueprints/Base/Enemy_BaseClass` _array_element))
        (bind (_enemy_to_spawn _cost_of_enemy) (`self.GetEnemySpawnInfo` _asenemy_base_class (defaults `/Game/TDRoR/Blueprints/SpawnPoints/SpawnManager` _asenemy_base_class)))
        (`BlueprintMapLibrary.Map_Add` (`self.Enemy List_InGame`) _enemy_to_spawn _cost_of_enemy)))
    (:`NewEnumerator1`
      (for _array_element_2 (`self.Enemies_Fire`)
        (bind _asenemy_base_class_2 (castclass `/Game/TDRoR/Enemy/Enemy_Blueprints/Base/Enemy_BaseClass` _array_element_2))
        (bind (_enemy_to_spawn_2 _cost_of_enemy_2) (`self.GetEnemySpawnInfo` _asenemy_base_class_2 (defaults `/Game/TDRoR/Blueprints/SpawnPoints/SpawnManager` _asenemy_base_class_2)))
        (`BlueprintMapLibrary.Map_Add` (`self.Enemy List_InGame`) _enemy_to_spawn_2 _cost_of_enemy_2)))
    (:`NewEnumerator2`
      (for _array_element_3 (`self.Enemies_Ice`)
        (bind _asenemy_base_class_3 (castclass `/Game/TDRoR/Enemy/Enemy_Blueprints/Base/Enemy_BaseClass` _array_element_3))
        (bind (_enemy_to_spawn_3 _cost_of_enemy_3) (`self.GetEnemySpawnInfo` _asenemy_base_class_3 (defaults `/Game/TDRoR/Blueprints/SpawnPoints/SpawnManager` _asenemy_base_class_3)))
        (`BlueprintMapLibrary.Map_Add` (`self.Enemy List_InGame`) _enemy_to_spawn_3 _cost_of_enemy_3)))
    (:`NewEnumerator3`
      (for _array_element_4 (`self.Enemies_Grass`)
        (bind _asenemy_base_class_4 (castclass `/Game/TDRoR/Enemy/Enemy_Blueprints/Base/Enemy_BaseClass` _array_element_4))
        (bind (_enemy_to_spawn_4 _cost_of_enemy_4) (`self.GetEnemySpawnInfo` _asenemy_base_class_4 (defaults `/Game/TDRoR/Blueprints/SpawnPoints/SpawnManager` _asenemy_base_class_4)))
        (`BlueprintMapLibrary.Map_Add` (`self.Enemy List_InGame`) _enemy_to_spawn_4 _cost_of_enemy_4))))
  (bind _keys (`BlueprintMapLibrary.Map_Keys` (`self.Enemy List_InGame`)))
  (for _array_element_5 _keys
    (bind _asenemy_base_class_5 (castclass `/Game/TDRoR/Enemy/Enemy_Blueprints/Base/Enemy_BaseClass` _array_element_5))
    (`KismetSystemLibrary.PrintString` (`KismetStringLibrary.Concat_StrStr` (`KismetSystemLibrary.GetClassDisplayName` _asenemy_base_class_5) " | " (`KismetStringLibrary.Conv_IntToString` (defaults `/Game/TDRoR/Blueprints/SpawnPoints/SpawnManager` _asenemy_base_class_5))))))

(fn `Calc Spawn Tokens`
  (locals (`Game Instance` :type "/Game/TDRoR/Blueprints/GameManagers/TDRoRInstance Object Reference") (Coeff :type "Float (double-precision)"))
  (bind _astdro_rinstance (cast `/Game/TDRoR/Blueprints/GameManagers/TDRoRInstance` (`GameplayStatics.GetGameInstance`)))
  (bind _output_get (set `local.Game Instance` _astdro_rinstance))
  (set `local.Coeff` (`/Game/TDRoR/Blueprints/GameManagers/TDRoRInstance.coeff` _output_get))
  (set `self.SpawnTokens` (`KismetMathLibrary.FTrunc` (+ (`KismetMathLibrary.Conv_IntToDouble` (`self.SpawnTokens`)) (* (`self.SpawnTokens`) (`local.Coeff`))))))

(fn `CheckRareEnironment`
  (returns (IsRare :type Boolean))
  ;[1 1 1] This should be in the map Spawner, but Testing right now here
  (if (<= (`KismetMathLibrary.RandomInteger` (`self.MaxRoll`)) (`self.RareChance`))
    (set `self.Rare_Variation` true)
    (`self.RareEvironment`)
    (else
      (set `self.Rare_Variation` false)))
  (return (`self.Rare_Variation`)))

(fn `GetAllSpawnPoints`
  (locals (Coeff :type "Float (double-precision)" :default 0.0) (`Game Instance` :type "/Game/TDRoR/Blueprints/GameManagers/TDRoRInstance Object Reference"))
  (bind _outactors (`GameplayStatics.GetAllActorsOfClass` "/Game/TDRoR/Blueprints/SpawnPoints/BP_SpawnPoint.BP_SpawnPoint_C"))
  (set `self.Spawn Points In Scene` _outactors))

(fn `GetEnemySpawnInfo`
  (params (EnemyClass :type "Actor Class Reference") (EnemySpawnCost :type Integer))
  (returns (`Enemy To Spawn` :type "Actor Class Reference") (`Cost of Enemy` :type Integer))
  (locals (TMP_EnemyClass :type "Actor Class Reference") (TMP_EnemySpawnCost :type Integer))
  (bind _output_get (set `local.TMP_EnemyClass` EnemyClass))
  (bind _output_get_2 (set `local.TMP_EnemySpawnCost` EnemySpawnCost))
  (return _output_get _output_get_2))

(fn `RemoveSpawnTokens`
  (params (`Enemy Cost` :type Integer))
  (set `self.SpawnTokens` (- (`self.SpawnTokens`) `Enemy Cost`)))

(fn `SpawnCheck`
  (locals (TempSpawner :type "/Game/TDRoR/Blueprints/SpawnPoints/BP_SpawnPoint Object Reference") (`Rand Int` :type Integer :default 0))
  (bind _enemy_list_ingame (`self.Enemy List_InGame`))
  (bind _tempspawner (`local.TempSpawner`))
  (for _array_element (`self.Spawn Points In Scene`)
    (bind _output_get (set `local.TempSpawner` _array_element))
    (if (and (`/Game/TDRoR/Blueprints/SpawnPoints/BP_SpawnPoint.IsSpawnerEnabled` _output_get) (`/Game/TDRoR/Blueprints/SpawnPoints/BP_SpawnPoint.BossNotDead` _output_get)) :!label _label
      (bind _values (`BlueprintMapLibrary.Map_Values` _enemy_list_ingame))
      (set `local.Rand Int` (`KismetMathLibrary.RandomInteger` (`KismetArrayLibrary.Array_Length` _values)))
      (bind _output (`|GetArrayItem` _values (`local.Rand Int`)))
      (if (>= (`self.SpawnTokens`) _output)
        (bind _keys (`BlueprintMapLibrary.Map_Keys` _enemy_list_ingame))
        (set `/Game/TDRoR/Blueprints/SpawnPoints/BP_SpawnPoint.Enemy To Spawn` (`|GetArrayItem` _keys (`local.Rand Int`)) _tempspawner)
        (`self.RemoveSpawnTokens` _output)
        (`/Game/TDRoR/Blueprints/SpawnPoints/BP_SpawnPoint.Spawn` _tempspawner)
        (elif (< (`self.SpawnTokens`) 5)
          (`KismetSystemLibrary.PrintString` "Cant Spawn")
          (else
            (goto _label))))
      (else
        (`KismetSystemLibrary.PrintString` "Cant Spawn")))))

(fn `UserConstructionScript`)