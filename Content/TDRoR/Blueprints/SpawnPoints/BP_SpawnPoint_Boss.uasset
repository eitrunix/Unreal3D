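; Boss spawn point that spawns the boss enemy at its own location when the game mode fires OnBossStart.
; On BeginPlay it binds to that event, then spawns only if no valid Boss exists and stores the new actor.
; SetupBoss picks the class by CurrentEnvironment, though all four environments currently map to BP_Enemy_BigSpooder.
; The construction script destroys the SpawnArea component after running the parent's script.
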(event `self.ReceiveBeginPlay`
  (`parent.ReceiveBeginPlay`)
  (bind _astdro_rgame_mode (cast `/Game/TDRoR/Blueprints/GameManagers/TDRoRGameMode` (`GameplayStatics.GetGameMode`)))
  (add `/Game/TDRoR/Blueprints/GameManagers/TDRoRGameMode.OnBossStart` _astdro_rgame_mode (delegate `BossSpawnEvent`)))

(event `BossSpawnEvent`
  (bind _scene (`self.Scene`))
  (`self.Boss`
    (:`then`)
    (:`else`
      (bind _boss (`self.SetupBoss` (`self.CurrentEnvironment`)))
      (bind _returnvalue (`|SpawnActorFromClass` _boss (`KismetMathLibrary.MakeTransform` (`SceneComponent.K2_GetComponentLocation` _scene) (`SceneComponent.K2_GetComponentRotation` _scene)) "AdjustIfPossibleButAlwaysSpawn" "OverrideRootScale" null null))
      (set `self.Boss` _returnvalue))))

(fn `GetEnvironment`
  (bind _astdro_rinstance (cast `/Game/TDRoR/Blueprints/GameManagers/TDRoRInstance` (`GameplayStatics.GetGameInstance`)))
  (set `self.CurrentEnvironment` (`/Game/TDRoR/Blueprints/GameManagers/TDRoRInstance.currentEnvironment` _astdro_rinstance)))

(fn `SetupBoss`
  (params (`Current Environment` :type "/Game/TDRoR/Blueprints/LevelGeneration/EnvironmentEnum Enum" :default "NewEnumerator0"))
  (returns (Boss :type "Actor Class Reference"))
  (return (select `/Game/TDRoR/Blueprints/LevelGeneration/EnvironmentEnum` `Current Environment` :`NewEnumerator0` "/Game/TDRoR/Enemies/Enemy_Great_Spider/BP_Enemy_BigSpooder.BP_Enemy_BigSpooder_C" :`NewEnumerator1` "/Game/TDRoR/Enemies/Enemy_Great_Spider/BP_Enemy_BigSpooder.BP_Enemy_BigSpooder_C" :`NewEnumerator2` "/Game/TDRoR/Enemies/Enemy_Great_Spider/BP_Enemy_BigSpooder.BP_Enemy_BigSpooder_C" :`NewEnumerator3` "/Game/TDRoR/Enemies/Enemy_Great_Spider/BP_Enemy_BigSpooder.BP_Enemy_BigSpooder_C" :!type "Actor Class Reference")))

(fn `UserConstructionScript`
  (`parent.UserConstructionScript`)
  (`ActorComponent.K2_DestroyComponent` (`self.SpawnArea`)))