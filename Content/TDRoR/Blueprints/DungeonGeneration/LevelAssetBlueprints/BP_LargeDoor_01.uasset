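; BP_LargeDoor_01 is an interactable double door among the dungeon generation level assets.
; OnInteract sets and returns the Opened flag, but only when CanBeOpened is true.
; While Opened is set, Tick calls OpenDoor, which uses RInterpTo to ease the left and right leaves toward fixed relative rotations.
; It has no closing logic, and Tick keeps interpolating after the doors reach their targets.
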(event `self.ReceiveTick`
  (params (DeltaSeconds :type "Float (single-precision)"))
  (if (`self.Opened`)
    (`self.Open Door` DeltaSeconds)))

(fn `OnInteract`
  (returns (Success :type Boolean))
  (if (`self.CanBeOpened`)
    (bind _output_get (set `self.Opened` true))
    (return _output_get)))

(fn `Open Door`
  (params (DeltaTime :type "Float (double-precision)"))
  (`SceneComponent.K2_SetRelativeRotation` (`self.Door_L`) (`KismetMathLibrary.RInterpTo` (`SceneComponent.RelativeRotation` (`self.Door_L`)) (struct :`Yaw` -30.0) DeltaTime 2.0) false false)
  (`SceneComponent.K2_SetRelativeRotation` (`self.Door_R`) (`KismetMathLibrary.RInterpTo` (`SceneComponent.RelativeRotation` (`self.Door_R`)) (struct :`Yaw` -150.0) DeltaTime 2.0) false false))

(fn `UserConstructionScript`)