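; Dungeon generator actor that runs map generation on BeginPlay to place modular 3x3 room Blueprints.
; Generate_Map spawns up to MaxRooms four-exit rooms in a loop, enabling each one's north exit.
; Each next spawn position is the last room mesh's relative location multiplied by RoomTileSize.
; The construction script can roll a new seed and seeds a random stream, which the spawn loop does not yet use.
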(event `self.ReceiveBeginPlay`
  (`self.Generate_Map`))

(event `Generate_Map`
  (for _ (range (`self.MaxRooms`))
    (set `self.PrevPosition` (`SceneComponent.GetRelativeTransform` (`self.CenterPoint`)))
    (bind _returnvalue (`|SpawnActorFromClass` "/Game/TDRoR/Blueprints/DungeonGeneration/Tiles/SM_MERGED_SM_Room_3x3_4Exits_Blueprint.SM_MERGED_SM_Room_3x3_4Exits_Blueprint_C" (`self.NewPosition`) "Undefined" "OverrideRootScale" null null))
    (`/Game/TDRoR/Blueprints/DungeonGeneration/Tiles/SM_MERGED_SM_Room_3x3_4Exits_Blueprint.Set Exits` _returnvalue true false false false)
    (bind _returnvalue_location (`KismetMathLibrary.BreakTransform` (`SceneComponent.GetRelativeTransform` (`StaticMeshActor.StaticMeshComponent` _returnvalue))))
    (set `self.NewPosition` (`KismetMathLibrary.MakeTransform` (* _returnvalue_location (`self.RoomTileSize`))))))

(fn `UserConstructionScript`
  (`|ExecutionSequence`
    (:`then_0`
      (if (`self.NewSeed`)
        (set `self.NewSeed` false)
        (bind _output_get (set `self.Seed` (`KismetMathLibrary.RandomInteger` 900000)))
        (`KismetMathLibrary.SetRandomStreamSeed` (`self.Stream`) _output_get)))
    (:`then_1`
      ;[1 1 1] Update Stream with Seed. Manual
      (`KismetMathLibrary.SetRandomStreamSeed` (`self.Stream`) (`self.Seed`)))))