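; Base collectable effect actor that scatters on spawn, then homes in on the player.
; BeginPlay teleports it by a random offset on each axis, bounded by MinDist and MaxDist.
; Tick moves it straight toward Target at Speed, falling back to the first player character when Target is invalid.
; It destroys itself on nearly reaching Target, using a location tolerance rather than overlap events, and grants nothing itself.
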(event `self.ReceiveBeginPlay`
  (bind _mindist (`self.MinDist`))
  (bind _maxdist (`self.MaxDist`))
  (`self.K2_SetActorLocation` (+ (`self.K2_GetActorLocation`) (`KismetMathLibrary.MakeVector` (`KismetMathLibrary.RandomFloatInRange` _mindist _maxdist) (`KismetMathLibrary.RandomFloatInRange` _mindist _maxdist) (`KismetMathLibrary.RandomFloatInRange` _mindist _maxdist)))))

(event `self.ReceiveTick`
  (params (DeltaSeconds :type "Float (single-precision)"))
  (bind _returnvalue (`self.K2_GetActorLocation`))
  (bind _target (`self.Target`)
    (:`then`
      (bind _returnvalue_2 (`self.K2_GetActorLocation` _target))
      (`self.K2_SetActorLocation` (+ (* (`KismetMathLibrary.Normal` (- _returnvalue_2 _returnvalue)) (* DeltaSeconds (`self.Speed`))) _returnvalue))
      (if (== _returnvalue_2 _returnvalue :`ErrorTolerance` 5.0)
        (`self.K2_DestroyActor`)))
    (:`else`
      (set `self.Target` (`GameplayStatics.GetPlayerCharacter` 0)))))

(fn `UserConstructionScript`)