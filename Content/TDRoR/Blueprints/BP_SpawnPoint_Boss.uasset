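; Boss spawn point actor that spawns the boss enemy when the game mode signals a boss start.
; On BeginPlay it binds its spawn event to the TDRoR game mode's OnBossStart event.
; That event calls SpawnEnemy at the Scene component's transform and stores the result in Boss, skipping if one is already valid.
; The construction script destroys the Sphere component.
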(event `self.ReceiveBeginPlay`
  (`parent.ReceiveBeginPlay`)
  (bind _astdro_rgame_mode (cast `/Game/TDRoR/Blueprints/GameManagers/TDRoRGameMode` (`GameplayStatics.GetGameMode`)))
  (add `/Game/TDRoR/Blueprints/GameManagers/TDRoRGameMode.OnBossStart` _astdro_rgame_mode (delegate `BossSpawnEvent`)))

(event `BossSpawnEvent`
  (bind _scene (`self.Scene`))
  (`self.Boss`
    (:`then`)
    (:`else`
      (bind _returnvalue (`SpawnPointComponent.SpawnEnemy` (`self.SpawnPoint`) (`SceneComponent.K2_GetComponentLocation` _scene) (`SceneComponent.K2_GetComponentRotation` _scene)))
      (set `self.Boss` _returnvalue))))

(fn `UserConstructionScript`
  (`parent.UserConstructionScript`)
  (`ActorComponent.K2_DestroyComponent` (`self.Sphere`)))