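; BP_LargeDoor_01 is a large double-door level actor meant to open when a Player_Base enters its trigger box.
; The overlap sets state flags and calls OpenDoor, which loops on two counters within one call, setting both doors' yaw.
; The counter-plus-rotation sums are unused, so the yaw variables never change there.
; OnInteract is empty, and the glow function only increments a timer, leaving its spotlight intensity call unreachable.
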(event `self.Box.OnComponentBeginOverlap`
  (params (OverlappedComponent :type "PrimitiveComponent Object Reference") (OtherActor :type "Actor Object Reference") (OtherComp :type "PrimitiveComponent Object Reference") (OtherBodyIndex :type Integer) (bFromSweep :type Boolean) (SweepResult :type "HitResult Structure (by ref)"))
  (cast `/Game/TDRoR/Player/Player_Base` OtherActor)
  (set `self.DoorsClosed` true)
  (set `self.PlayerInteracted` true)
  (`self.OpenDoor`))

(fn `Light_Glow_Effect`
  (locals (Light_Intensity :type "Float (double-precision)" :default 0.0) (Timer :type "Float (double-precision)") (Trigger :type Boolean :default true))
  (if (`local.Trigger`)
    (`/Engine/EditorBlueprintResources/StandardMacros.IncrementFloat` (`local.Timer`))))

(fn `OnInteract`
  (returns (Success :type Boolean)))

(fn `OpenDoor`
  (bind _dooropentimer01 (`self.DoorOpenTimer01`))
  (bind _dooropentimer02 (`self.DoorOpenTimer02`))
  (while (and (<= _dooropentimer02 -20.0) (>= _dooropentimer01 20.0))
    (bind _result (`/Engine/EditorBlueprintResources/StandardMacros.IncrementFloat` _dooropentimer01)
      (:`  `
        (bind _result_2 (`/Engine/EditorBlueprintResources/StandardMacros.DecrementFloat` _dooropentimer02)
          (:`  `
            (`SceneComponent.K2_SetRelativeRotation` (`self.Door_L`) (`KismetMathLibrary.MakeRotator` 0.0 0.0 (`self.Door_L_Rotation`)) false false)
            (`SceneComponent.K2_SetRelativeRotation` (`self.Door_R`) (`KismetMathLibrary.MakeRotator` 0.0 0.0 (`self.Door_R_Rotation`)) false false)))))))

(fn `UserConstructionScript`)