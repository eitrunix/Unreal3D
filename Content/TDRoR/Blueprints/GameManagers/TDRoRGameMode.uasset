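; TDRoRGameMode is the game mode, with a ShowStats event that prints the player's stats on screen as a debug readout.
; ShowStats casts the game instance to TDRoRInstance and loops over the keys of its PlayerStats1 map, pairing each with the value at the same index.
; Each enum name and value is shown through a timed PrintString.
; Tick and the construction script are empty.
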(event `self.ReceiveTick`
  (params (DeltaSeconds :type "Float (single-precision)")))

(event `ShowStats`
  (bind _astdro_rinstance (cast `/Game/TDRoR/Blueprints/GameManagers/TDRoRInstance` (`GameplayStatics.GetGameInstance`)))
  (bind _playerstats_1 (`/Game/TDRoR/Blueprints/GameManagers/TDRoRInstance.PlayerStats_1` _astdro_rinstance))
  (bind _keys (`BlueprintMapLibrary.Map_Keys` _playerstats_1))
  (for (_array_element _array_index) _keys
    (bind _values (`BlueprintMapLibrary.Map_Values` _playerstats_1))
    (bind (_output_count _output_value) (break `/Game/TDRoR/Items/FStatData` (`|GetArrayItem` _values _array_index)))
    (`KismetSystemLibrary.PrintString` (`KismetStringLibrary.Concat_StrStr` (`|GetEnumeratorNameAsString` _array_element) ": " (`KismetStringLibrary.Conv_DoubleToString` _output_value)) true true (struct :`G` 0.66 :`B` 1.0 :`A` 1.0) 10.0)))

(fn `UserConstructionScript`)