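; Game instance for TDRoR that holds run-wide state: currency, XP and level, a keyed player stat map, the master item list and stage progress.
; A 0.1-second Delay loop drives the game clock and recomputes a difficulty coefficient from player count, minutes, difficulty and stages completed.
; Clock milestones notify the SpawnManager to run its 10-second timer or recalculate spawn tokens.
; Level completion increments the stage count and opens the next of three looping levels.
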(event `/Game/TDRoR/Blueprints/GameManagers/BPI_Interact.Gain Currency Event`
  (params (Amount :type Integer))
  (`self.SetCurrency` (+ Amount (`self.currentCurrency`))))

(event `/Game/TDRoR/Blueprints/GameManagers/BPI_Interact.Take Currency Event`
  (params (Ammount :type Integer))
  (`self.SetCurrency` (- (`self.currentCurrency`) Ammount)))

(event `Set Stats`
  (bind _asdrongo_player_character (cast `/Game/Characters/Heroes/Drongo/DrongoPlayerCharacter` (`GameplayStatics.GetPlayerPawn` 0)))
  (`|ExecutionSequence`
    (:`then_0`
      (`self.SetPlayerStat` (`/Game/Characters/Heroes/Drongo/DrongoPlayerCharacter.Health` _asdrongo_player_character)))
    (:`then_1`
      (`self.SetPlayerStat` (`/Game/Characters/Heroes/Drongo/DrongoPlayerCharacter.Damage` _asdrongo_player_character) "Damage"))
    (:`then_2`
      (`self.SetPlayerStat` (`/Game/Characters/Heroes/Drongo/DrongoPlayerCharacter.FireRate` _asdrongo_player_character) "FireRate"))
    (:`then_3`
      (`self.SetPlayerStat` (`/Game/Characters/Heroes/Drongo/DrongoPlayerCharacter.MaxHealth` _asdrongo_player_character) "MaxHealth"))))

(event `self.ReceiveInit`
  (`|ExecutionSequence`
    (:`then_0`
      (add `self.3Minutemark` (delegate `3 Minute Update`))
      (`self.SetupMasterItemList`))
    (:`then_1`
      (add `self.LevelComplete` (delegate `EndOfLevelEvent`)))
    (:`then_2`
      ;[1 1 1] Game Time Events
      (`|ExecutionSequence`
        (:`then_0`
          (add `self.StartTimer` (delegate `Start Game Time`)))
        (:`then_1`
          (add `self.PauseTimer` (delegate `Pause Game time`)))
        (:`then_2`
          (add `self.ResetTimer` (delegate `Reset Game time`)))
        (:`then_3`
          (add `self.10SecondMark` (delegate `10SecondEvent`)))))))

(event `3 Minute Update`
  (bind _returnvalue (`GameplayStatics.GetActorOfClass` "/Game/TDRoR/Blueprints/SpawnPoints/SpawnManager.SpawnManager_C"))
  (`/Game/TDRoR/Blueprints/SpawnPoints/SpawnManager.Calc Spawn Tokens` _returnvalue))

(event `EndOfLevelEvent`
  (bind _currentstage (`self.currentStage`))
  (`|ExecutionSequence`
    (:`then_0`
      (bind _output_get (set `self.currentStage` (+ _currentstage 1)))
      (if (== _output_get 4)
        (set `self.currentStage` 1)))
    (:`then_1`
      (set `self.stagesCompleted` (+ (`self.stagesCompleted`) 1)))
    (:`then_2`
      (`GameplayStatics.OpenLevel` (`KismetStringLibrary.Conv_StringToName` (`KismetStringLibrary.Concat_StrStr` "Level" (`KismetStringLibrary.Conv_IntToString` _currentstage)))))))

(event `Start Game Time`
  ;[1 1 1] Game Time Events
  (set `self.GameTimeRunning` true)
  (`KismetSystemLibrary.Delay` 0.1 :!label _label)
  (`self.CalcCoeff`)
  (`self.CalcTimeInGame`)
  (if (`self.GameTimeRunning`)
    (goto _label)))

(event `Pause Game time`
  ;[1 1 1] Game Time Events
  (set `self.GameTimeRunning` false))

(event `Reset Game time`
  ;[1 1 1] Game Time Events
  (set `self.gameTimeInMilliseconds` 0)
  (set `self.gameTimeInSeconds` 0)
  (set `self.gameTimeInMinutes` 0)
  (set `self.TempGameTime` 0))

(event `10SecondEvent`
  ;[1 1 1] Game Time Events
  (bind _returnvalue (`GameplayStatics.GetActorOfClass` "/Game/TDRoR/Blueprints/SpawnPoints/SpawnManager.SpawnManager_C"))
  (`/Game/TDRoR/Blueprints/SpawnPoints/SpawnManager.10SecondTimer` _returnvalue))

(fn `AddPlayerLevel`
  (returns (Output_Get :type Integer))
  (bind _output_get (set `self.playerLevel` (+ (`self.playerLevel`) 1)))
  (return _output_get))

(fn `addStageComplete`
  (set `self.stagesCompleted` (+ (`self.stagesCompleted`) 1)))

(fn `AddToExp`
  (params (ExpGiven :type Integer))
  (bind _output_get (set `self.playerExp` (+ (`self.playerExp`) ExpGiven)))
  (if (>= _output_get (`self.playerExpNextLevel`))
    (`self.AddPlayerLevel`)))

(fn `CalcCoeff`
  (returns (Coeff :type "Float (double-precision)"))
  (`self.CalcPlayerFactor`)
  (`self.CalcDifficultyValue`)
  (`self.CalcTimeFactor`)
  (`self.CalcStageFactor`)
  (bind _output_get (set `self.coeff` (* (* (+ (`self.playerFactor`) (`KismetMathLibrary.Conv_IntToDouble` (`self.gameTimeInMinutes`))) (`self.timeFactor`)) (`self.stageFactor`))))
  (return _output_get))

(fn `CalcDifficultyValue`
  (set `self.difficultyValue` (select `/Game/TDRoR/Blueprints/GameManagers/Difficulty` (`self.Difficulty`) :`NewEnumerator0` 1.0 :`NewEnumerator1` 2.0 :`NewEnumerator2` 3.0 :!type "Float (single-precision)")))

(fn `CalcPlayerFactor`
  (set `self.playerFactor` (* (`self.playerCount`) (+ 1.0 (`self.PlayerMod`)))))

(fn `CalcStageFactor`
  (set `self.stageFactor` (`KismetMathLibrary.MultiplyMultiply_FloatFloat` (`self.StageMod`) (`KismetMathLibrary.Conv_IntToDouble` (`self.stagesCompleted`)))))

(fn `CalcTimeFactor`
  (set `self.timeFactor` (* (`KismetMathLibrary.MultiplyMultiply_FloatFloat` (`KismetMathLibrary.Conv_IntToDouble` (`self.playerCount`)) 0.2) (* (`self.timeMod`) (`self.difficultyValue`)))))

(fn `CalcTimeInGame`
  (locals (TempSeconds :type "Float (double-precision)" :default 0.0))
  (`/Engine/EditorBlueprintResources/StandardMacros.IncrementInt` (`self.gameTimeInMilliseconds`)
    (:`  `
      (if (== (`self.gameTimeInMilliseconds`) 10)
        (`|ExecutionSequence`
          (:`then_0`
            (set `self.gameTimeInMilliseconds` 0)
            (`/Engine/EditorBlueprintResources/StandardMacros.IncrementInt` (`self.gameTimeInSeconds`)
              (:`  `
                (`/Engine/EditorBlueprintResources/StandardMacros.IncrementInt` (`self.10 SecondInterval`)))))
          (:`then_1`
            (if (>= (`self.10 SecondInterval`) 10)
              (set `self.10 SecondInterval` 0)
              (`self.10SecondMark`)))
          (:`then_2`
            (if (== (`self.gameTimeInSeconds`) 60)
              (set `self.gameTimeInSeconds` 0)
              (`/Engine/EditorBlueprintResources/StandardMacros.IncrementInt` (`self.gameTimeInMinutes`)
                (:`  `
                  (bind _result (`/Engine/EditorBlueprintResources/StandardMacros.IncrementInt` (`self.TempGameTime`))
                    (:`  `
                      (if (>= _result (`self.TimeBeforeSpawnUpdate`))
                        (set `self.TempGameTime` 0)
                        (`self.3Minutemark`)
                        (`KismetSystemLibrary.PrintString` (`KismetStringLibrary.Concat_StrStr` "3 minutes Passed" "  |  " "Total Time = " (`KismetStringLibrary.Conv_IntToString` (`self.gameTimeInMinutes`))))))))))))))))

(fn `GetEnemiesOnStage`
  (returns (enemiesOnStage :type Integer))
  (return (`self.enemiesOnStage`)))

(fn `GetMaxEnemiesOnStage`
  (returns (MAX_ENEMIES :type Integer))
  (return (`self.MAX_ENEMIES`)))

(fn `GetPlayerStat`
  (params (Key :type "statToIncrease Enum" :default "Health"))
  (returns (Count :type Integer) (Value :type "Float (double-precision)"))
  (bind (_value _returnvalue) (`BlueprintMapLibrary.Map_Find` (`self.PlayerStats_1`) Key))
  (if _returnvalue
    (return (break `/Game/TDRoR/Items/FStatData` _value) (`.Value_4_518043764B4C229A88019B9BFC888E2C` (break `/Game/TDRoR/Items/FStatData` _value)))
    (else
      (`KismetSystemLibrary.PrintString` (`KismetStringLibrary.Concat_StrStr` "TDRoRInstance: Variable PlayerStats is missing : " (`|GetEnumeratorNameAsString` Key)) true true (struct :`R` 1.0 :`B` 0.002103 :`A` 1.0) 300.0))))

(fn `OnInteract`
  (returns (Success :type Boolean))
  (return false))

(fn `SetArmor`
  (params (currentPlayerArmor :type "Float (double-precision)"))
  (`self.SetPlayerStat` currentPlayerArmor "Armour"))

(fn `SetCurrency`
  (params (ChangeInTotal :type Integer))
  (returns (`New Total Value` :type Integer))
  (bind _output_get (set `self.currentCurrency` ChangeInTotal))
  (`KismetSystemLibrary.PrintString` (`KismetStringLibrary.Conv_IntToString` _output_get))
  (return _output_get))

(fn `SetDamage`
  (params (currentPlayerDamage :type "Float (double-precision)"))
  (`self.SetPlayerStat` currentPlayerDamage "Damage"))

(fn `SetEnemiesOnStage`
  (params (enemiesOnStage :type Integer))
  (set `self.enemiesOnStage` enemiesOnStage))

(fn `SetFireRate`
  (params (currentPlayerFireRate :type "Float (double-precision)"))
  (`self.SetPlayerStat` currentPlayerFireRate "FireRate"))

(fn `SetHealth`
  (params (currentPlayerHealth :type "Float (double-precision)"))
  (`self.SetPlayerStat` currentPlayerHealth))

(fn `SetMaxEnemiesOnStage`
  (params (MAX_ENEMIES :type Integer))
  (set `self.MAX_ENEMIES` MAX_ENEMIES))

(fn `SetMoveSpeed`
  (params (currentPlayerMoveSpeed :type "Float (double-precision)"))
  (`self.SetPlayerStat` currentPlayerMoveSpeed "MoveSpeed"))

(fn `SetPlayerStat`
  (params (NewStat :type "Float (double-precision)") (Key :type "statToIncrease Enum" :default "Health"))
  (bind _playerstats_1 (`self.PlayerStats_1`))
  (bind (_value _returnvalue) (`BlueprintMapLibrary.Map_Find` _playerstats_1 Key))
  (if _returnvalue
    (bind _result (`/Engine/EditorBlueprintResources/StandardMacros.IncrementInt` (break `/Game/TDRoR/Items/FStatData` _value))
      (:`  `
        (`BlueprintMapLibrary.Map_Add` _playerstats_1 Key (make `/Game/TDRoR/Items/FStatData` _result NewStat))
        (`self.StatIncreased` Key)))
    (else
      (`KismetSystemLibrary.PrintString` (`KismetStringLibrary.Concat_StrStr` "TDRoRInstance: Variable PlayerStats is missing : " (`|GetEnumeratorNameAsString` Key)) true true (struct :`R` 1.0 :`B` 0.002103 :`A` 1.0) 300.0))))

(fn `SetStage`
  (params (currentStage :type Integer))
  (set `self.currentStage` currentStage))

(fn `SetupEnvironment`
  (params (currentEnvironment :type "/Game/TDRoR/Blueprints/LevelGeneration/EnvironmentEnum Enum" :default "NewEnumerator0"))
  (locals (randInt :type Integer :default 0))
  (set `self.currentEnvironment` currentEnvironment))

(fn `SetupMasterItemList`
  (set `self.MasterItemList` (`|MakeArray` "/Game/TDRoR/Items/BP_ArmorPickup.BP_ArmorPickup_C" "/Game/TDRoR/Items/BP_ArmorSprintingPickup.BP_ArmorSprintingPickup_C" "/Game/TDRoR/Items/BP_BleedPickup.BP_BleedPickup_C" "/Game/TDRoR/Items/BP_CritPickUp.BP_CritPickUp_C" "/Game/TDRoR/Items/BP_DamagePickup.BP_DamagePickup_C" "/Game/TDRoR/Items/BP_FireRatePickup.BP_FireRatePickup_C" "/Game/TDRoR/Items/BP_HealthPickup.BP_HealthPickup_C" "/Game/TDRoR/Items/BP_MoveSpeedPickup.BP_MoveSpeedPickup_C" "/Game/TDRoR/Items/BP_OnHitPickUp.BP_OnHitPickUp_C" "/Game/TDRoR/Items/BP_OnKillPickup.BP_OnKillPickup_C" "/Game/TDRoR/Items/BP_OvertimeHealNoCombatPickup.BP_OvertimeHealNoCombatPickup_C" "/Game/TDRoR/Items/BP_OvertimeHealPickup.BP_OvertimeHealPickup_C" "/Game/TDRoR/Items/BP_SprintSpeedPickup.BP_SprintSpeedPickup_C" :!type "Actor Class Reference")))