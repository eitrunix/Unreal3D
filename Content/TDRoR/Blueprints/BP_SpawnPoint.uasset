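; BP_SpawnPoint is an enemy spawner that runs while the player is inside its sphere and the boss is alive.
; Tick spawns an enemy through the SpawnPoint component, increments the stage count on TDRoRInstance and fires a spawned event.
; That event disables the spawner once the count exceeds the stage maximum, otherwise starts a timer that re-allows spawning.
; A game mode boss-finish dispatcher, rebound every active Tick, stops spawning.
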(event `SpawnedAnEnemy_Event`
  (bind _astdro_rinstance (cast `/Game/TDRoR/Blueprints/GameManagers/TDRoRInstance` (`GameplayStatics.GetGameInstance`)))
  (`|ExecutionSequence`
    (:`then_0`
      (bind _max_enemies (`/Game/TDRoR/Blueprints/GameManagers/TDRoRInstance.GetMaxEnemiesOnStage` _astdro_rinstance))
      (set `self.TotalEnemiesSpawnabl` _max_enemies))
    (:`then_1`
      (bind _enemiesonstage (`/Game/TDRoR/Blueprints/GameManagers/TDRoRInstance.GetEnemiesOnStage` _astdro_rinstance))
      (set `self.EnemiesSpawned` _enemiesonstage))
    (:`then_2`
      (if (> (`self.EnemiesSpawned`) (`self.TotalEnemiesSpawnabl`))
        (set `self.IsSpawnerEnabled` false)
        (`KismetSystemLibrary.PrintString` "End Of Spawning")
        (else
          (`KismetSystemLibrary.K2_SetTimerDelegate` (delegate `SpawnTimer`) (`self.TestTimer`)))))))

(event `SpawnTimer`
  (set `self.CanSpawn` true))

(event `Stop Spawning`
  ;[1 1 1] Turn Off Spawning when the Boss is Dead
  (set `self.BossNotDead` false))

(event `self.ReceiveTick`
  (params (DeltaSeconds :type "Float (single-precision)"))
  (bind _scene (`self.Scene`))
  (if (and (`self.IsSpawnerEnabled`) (`self.BossNotDead`))
    (`|ExecutionSequence`
      (:`then_0`
        (add `self.SpawnedAnEnemy` (delegate `SpawnedAnEnemy_Event`)))
      (:`then_1`
        ;[1 1 1] Turn Off Spawning when the Boss is Dead
        (bind _astdro_rgame_mode (cast `/Game/TDRoR/Blueprints/GameManagers/TDRoRGameMode` (`GameplayStatics.GetGameMode`)))
        (add `/Game/TDRoR/Blueprints/GameManagers/TDRoRGameMode.OnBossFinish` _astdro_rgame_mode (delegate `Stop Spawning`)))
      (:`then_2`
        ;[1 1 1] Set the Location and Rotation for the Enemy to Spawn At, Spawn Enemy Picks an enemy from an Array, and spawns that enemy
        (if (`self.CanSpawn`)
          (set `self.CanSpawn` false)
          (`SpawnPointComponent.SpawnEnemy` (`self.SpawnPoint`) (`SceneComponent.K2_GetComponentLocation` _scene) (`SceneComponent.K2_GetComponentRotation` _scene))
          (bind _astdro_rinstance (cast `/Game/TDRoR/Blueprints/GameManagers/TDRoRInstance` (`GameplayStatics.GetGameInstance`)))
          (bind _enemiesonstage (`/Game/TDRoR/Blueprints/GameManagers/TDRoRInstance.GetEnemiesOnStage` _astdro_rinstance))
          (`/Game/TDRoR/Blueprints/GameManagers/TDRoRInstance.SetEnemiesOnStage` _astdro_rinstance (+ _enemiesonstage 1))
          (`self.SpawnedAnEnemy`)
          (`KismetSystemLibrary.PrintString` "Enemy Spawned"))))))

(event `self.Sphere.OnComponentBeginOverlap`
  (params (OverlappedComponent :type "PrimitiveComponent Object Reference") (OtherActor :type "Actor Object Reference") (OtherComp :type "PrimitiveComponent Object Reference") (OtherBodyIndex :type Integer) (bFromSweep :type Boolean) (SweepResult :type "HitResult Structure (by ref)"))
  (cast `/Game/TDRoR/Characters/Heroes/Drongo/DrongoPlayerCharacter` OtherActor)
  (set `self.IsSpawnerEnabled` true))

(event `self.Sphere.OnComponentEndOverlap`
  (params (OverlappedComponent :type "PrimitiveComponent Object Reference") (OtherActor :type "Actor Object Reference") (OtherComp :type "PrimitiveComponent Object Reference") (OtherBodyIndex :type Integer))
  (cast `/Game/TDRoR/Characters/Heroes/Drongo/DrongoPlayerCharacter` OtherActor)
  (set `self.IsSpawnerEnabled` false))

(fn `UserConstructionScript`)