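; BP_RoomTile_Base is a base dungeon-generation room tile that places a door or wall on each of its four sides.
; The construction script runs SetupRoomExits, which calls SpawnExits once per RoomData key, redundantly rebuilding every side each time.
; SpawnExits maps value order to West, East, South and North connection components, setting mesh and some yaw rotations by axis.
; BuildExits is an empty stub, and SetExits only prints debug text.
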(fn `Build_Exits`)

(fn `Set_Exits`
  (bind _keys (`BlueprintMapLibrary.Map_Keys` (`self.RoomData`)))
  (for (_ _array_index) _keys
    (bind _values (`BlueprintMapLibrary.Map_Values` (`self.RoomData`)))
    (if (`|GetArrayItem` _values _array_index)
      (`KismetSystemLibrary.PrintString` "West Can Leave")
      (else
        (`KismetSystemLibrary.PrintString` "West Cant Leave")))))

(fn `Setup_Room_Exits`
  (bind _roomdata (`self.RoomData`))
  (bind _keys (`BlueprintMapLibrary.Map_Keys` _roomdata))
  (for _array_element _keys
    (if (`BlueprintMapLibrary.Map_Contains` _roomdata _array_element)
      (`self.Spawn_Exits`))))

(fn `Spawn_Exits`
  (locals (NewLocalVar_0 :type "StaticMesh Object Reference") (Current_Pos :type Integer))
  (bind _wall_mesh (`self.Wall_Mesh`))
  (bind _door_mesh (`self.Door_Mesh`))
  (bind _values (`BlueprintMapLibrary.Map_Values` (`self.RoomData`)))
  (for (_array_element _array_index) _values
    (bind _output_get (set `local.Current_Pos` _array_index))
    (if _array_element
      (if (<= _array_index 1)
        (bind _returnvalue (select `int` _output_get :`0` (`self.W_Connection`) :`1` (`self.E_Connection`) :`2` (`self.S_Connection`) :`3` (`self.N_Connection`)))
        (`StaticMeshComponent.SetStaticMesh` _returnvalue _door_mesh)
        (else
          (`StaticMeshComponent.SetStaticMesh` _returnvalue _door_mesh)
          (`SceneComponent.K2_SetRelativeRotation` _returnvalue (struct :`Yaw` 90.0) false false)))
      (elif (<= _array_index 1)
        (`StaticMeshComponent.SetStaticMesh` _returnvalue _wall_mesh)
        (`SceneComponent.K2_SetRelativeRotation` _returnvalue (struct :`Yaw` 90.0) false false)
        (else
          (`StaticMeshComponent.SetStaticMesh` _returnvalue _wall_mesh))))))

(fn `UserConstructionScript`
  (`self.Setup_Room_Exits`)
  (`self.Build_Exits`))