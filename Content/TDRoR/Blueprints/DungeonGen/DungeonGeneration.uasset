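; Dungeon generator actor that spawns a seeded random sequence of start, transition, boss and end rooms on BeginPlay.
; SetupRoomLocations walks a square grid calling SpawnTiles, which picks each room's directional variant by running count until the room limit is reached.
; Only the first room uses its grid position; later rooms use NewLocation, which is never set here.
; TIleSpawn reads each room's exits, but SpawnTiles ignores them; debug prints list the results.
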(event `self.ReceiveBeginPlay`
  (`KismetMathLibrary.SeedRandomStream` (`self.Seed`))
  (`self.Setup_Dungeon`))

(fn `AddTilesToRoomList`
  (params (`Rooms To Spawn` :type Integer))
  (locals (TmpRoom :type "/Game/TDRoR/Blueprints/DungeonGen/BP_RoomTile_Base Class Reference") (LoopComplete :type Boolean :default true))
  (`|ExecutionSequence`
    (:`then_0`
      (`KismetArrayLibrary.Array_Add` (`self.Dungeon_Tiles`) (`self.StartRoom`)))
    (:`then_1`
      (for _ (range `Rooms To Spawn`)
        (`KismetArrayLibrary.Array_Add` (`self.Dungeon_Tiles`) (`self.TransitionTile`)))
      (set `local.LoopComplete` true))
    (:`then_2`
      (if (`local.LoopComplete`)
        (`KismetArrayLibrary.Array_Add` (`self.Dungeon_Tiles`) (`self.BossRoom`))
        (`KismetArrayLibrary.Array_Add` (`self.Dungeon_Tiles`) (`self.EndRoom`))))))

(fn `DebugDungon`
  (bind _tile_locations (`self.Tile_Locations`))
  (`|ExecutionSequence`
    (:`then_0`
      (bind _keys (`BlueprintMapLibrary.Map_Keys` _tile_locations))
      (for _array_element _keys
        (`KismetSystemLibrary.PrintString` (`KismetStringLibrary.Conv_IntVectorToString` _array_element))))
    (:`then_1`
      (bind _values (`BlueprintMapLibrary.Map_Values` _tile_locations))
      (for _array_element_2 _values
        (`KismetSystemLibrary.PrintString` (`KismetSystemLibrary.GetClassDisplayName` _array_element_2))))))

(fn `Setup_Dungeon`
  (`|ExecutionSequence`
    (:`then_0`
      (`self.AddTilesToRoomList` (`self.# of Rooms to Spawn`)))
    (:`then_1`
      (`self.Setup_Room_Locations`))
    (:`then_2`
      (`self.DebugDungon`))))

(fn `Setup_Room_Locations`
  (locals (Tile_Size :type "Float (double-precision)" :default 2400.0) (Temp_TileLocation :type "Vector Structure"))
  (bind _tile_size (`local.Tile_Size`))
  (bind _returnvalue (- (`self.# of Rooms to Spawn`) 1))
  (for _index (range (+ _returnvalue 1))
    (for _index_2 (range (+ _returnvalue 1))
      (`BlueprintMapLibrary.Map_Add` (`self.Tile_Locations`) (make `IntVector` _index _index_2))
      (bind _returnvalue_2 (* _tile_size (`KismetMathLibrary.Conv_IntToDouble` _index)))
      (bind _returnvalue_3 (* _tile_size (`KismetMathLibrary.Conv_IntToDouble` _index_2)))
      (set `local.Temp_TileLocation` (`KismetMathLibrary.MakeVector` _returnvalue_2 _returnvalue_3))
      (`self.Spawn Tiles` (`KismetMathLibrary.MakeTransform` (`KismetMathLibrary.MakeVector` _returnvalue_2 _returnvalue_3))))))

(fn `Spawn Tiles`
  (params (`Spawn Location` :type "Transform Structure") (`Tile Location` :type "IntVector Structure"))
  (locals (TmpNum :type Integer :default 0) (RoomToSpawn :type "/Game/TDRoR/Blueprints/DungeonGen/BP_RoomTile_Base Class Reference") (CurrentLocation :type "Transform Structure") (Prev_Location :type "Transform Structure") (New_Location :type "Transform Structure") (ExitLocations :type "Array of Transform Structure") (`Direction of Exit` :type Integer :default 0) (TmpLocation :type "IntVector Structure") (XPos :type "Float (double-precision)" :default 0.0) (YPos :type "Float (double-precision)" :default 0.0))
  (bind _roomcount (`self.RoomCount`))
  (bind _roomtospawn (`local.RoomToSpawn`))
  (set `local.CurrentLocation` `Spawn Location`)
  (if (<= _roomcount (`self.# of Rooms to Spawn`))
    (if (== _roomcount 0)
      (set `self.StartTilePlaced` true)
      (set `self.StartRoom` (select `int` (`KismetMathLibrary.RandomIntegerFromStream` 4 (`self.Seed`)) :`0` "/Game/TDRoR/Blueprints/DungeonGen/StartRooms/BP_StartRoom_N.BP_StartRoom_N_C" :`1` "/Game/TDRoR/Blueprints/DungeonGen/StartRooms/BP_StartRoom_S.BP_StartRoom_S_C" :`2` "/Game/TDRoR/Blueprints/DungeonGen/StartRooms/BP_StartRoom_E.BP_StartRoom_E_C" :`3` "/Game/TDRoR/Blueprints/DungeonGen/StartRooms/BP_StartRoom_W.BP_StartRoom_W_C" :!type "/Game/TDRoR/Blueprints/DungeonGen/BP_RoomTile_Base Class Reference"))
      (set `local.RoomToSpawn` (`self.StartRoom`))
      (else
        (set `local.CurrentLocation` (`local.New_Location`))
        (if (and (`self.StartTilePlaced`) (== (`self.RoomCount`) (- (`self.# of Rooms to Spawn`) 1)))
          (set `self.BossRoom` (select `int` (`KismetMathLibrary.RandomIntegerFromStream` 4 (`self.Seed`)) :`0` "/Game/TDRoR/Blueprints/DungeonGen/BossRoom/BP_BossRoom_N.BP_BossRoom_N_C" :`1` "/Game/TDRoR/Blueprints/DungeonGen/BossRoom/BP_BossRoom_S.BP_BossRoom_S_C" :`2` "/Game/TDRoR/Blueprints/DungeonGen/BossRoom/BP_BossRoom_E.BP_BossRoom_E_C" :`3` "/Game/TDRoR/Blueprints/DungeonGen/BossRoom/BP_BossRoom_E.BP_BossRoom_E_C" :!type "/Game/TDRoR/Blueprints/DungeonGen/BP_RoomTile_Base Class Reference"))
          (set `local.RoomToSpawn` (`self.BossRoom`))
          (elif (== (`self.RoomCount`) (`self.# of Rooms to Spawn`))
            (set `self.EndRoom` (select `int` (`KismetMathLibrary.RandomIntegerFromStream` 4 (`self.Seed`)) :`0` "/Game/TDRoR/Blueprints/DungeonGen/EndRoom/BP_EndRoom_N.BP_EndRoom_N_C" :`1` "/Game/TDRoR/Blueprints/DungeonGen/EndRoom/BP_EndRoom_S.BP_EndRoom_S_C" :`2` "/Game/TDRoR/Blueprints/DungeonGen/EndRoom/BP_EndRoom_E.BP_EndRoom_E_C" :`3` "/Game/TDRoR/Blueprints/DungeonGen/EndRoom/BP_EndRoomW.BP_EndRoomW_C" :!type "/Game/TDRoR/Blueprints/DungeonGen/BP_RoomTile_Base Class Reference"))
            (set `local.RoomToSpawn` (`self.EndRoom`))
            (else
              (set `self.TransitionTile` (select `int` (`KismetMathLibrary.RandomIntegerFromStream` 4 (`self.Seed`)) :`0` "/Game/TDRoR/Blueprints/DungeonGen/TransitionRooms/BP_TransitionRoom_NS.BP_TransitionRoom_NS_C" :`1` "/Game/TDRoR/Blueprints/DungeonGen/TransitionRooms/BP_TransitionRoom_NS.BP_TransitionRoom_NS_C" :`2` "/Game/TDRoR/Blueprints/DungeonGen/TransitionRooms/BP_TransitionRoom_EW.BP_TransitionRoom_EW_C" :`3` "/Game/TDRoR/Blueprints/DungeonGen/TransitionRooms/BP_TransitionRoom_EW.BP_TransitionRoom_EW_C" :!type "/Game/TDRoR/Blueprints/DungeonGen/BP_RoomTile_Base Class Reference"))
              (set `local.RoomToSpawn` (`self.TransitionTile`)))))))
    (`/Engine/EditorBlueprintResources/StandardMacros.IncrementInt` (`self.RoomCount`)
      (:`  `
        (bind _values (`BlueprintMapLibrary.Map_Values` (`self.Tile_Locations`)))
        (`KismetArrayLibrary.Array_Add` _values _roomtospawn)
        (`KismetSystemLibrary.PrintString` (`KismetSystemLibrary.GetClassDisplayName` _roomtospawn))
        (`self.TIleSpawn` _roomtospawn (`local.CurrentLocation`))))))

(fn `StartRoomSelect`)

(fn `TIleSpawn`
  (params (`Room To Spawn` :type "Actor Class Reference") (SpawnTransform :type "Transform Structure"))
  (returns (`North?` :type Boolean) (`South?` :type Boolean) (`East?` :type Boolean) (`West?` :type Boolean))
  (locals (ExitLocations :type "Array of Transform Structure") (NorthExit :type Boolean) (SouthExit :type Boolean) (EastExit :type Boolean) (WestExit :type Boolean))
  (bind _returnvalue (`|SpawnActorFromClass` `Room To Spawn` SpawnTransform "Undefined" "OverrideRootScale" null null))
  (bind _asbp_room_tile_base (cast `/Game/TDRoR/Blueprints/DungeonGen/BP_RoomTile_Base` _returnvalue))
  (`/Game/TDRoR/Blueprints/DungeonGen/BP_RoomTile_Base.Setup_Room_Exits` _asbp_room_tile_base)
  (bind _values (`BlueprintMapLibrary.Map_Values` (`/Game/TDRoR/Blueprints/DungeonGen/BP_RoomTile_Base.RoomData` _asbp_room_tile_base)))
  (for (_array_element _array_index) _values
    (switch `int` _array_index
      (:`0`
        (if _array_element
          (set `local.WestExit` true)
          (break)
          (else
            (set `local.WestExit` false))))
      (:`1`
        (if _array_element
          (set `local.EastExit` true)
          (break)
          (else
            (set `local.EastExit` false))))
      (:`2`
        (if _array_element
          (set `local.SouthExit` true)
          (break)
          (else
            (set `local.SouthExit` false))))
      (:`3`
        (if _array_element
          (set `local.NorthExit` true)
          (break)
          (else
            (set `local.NorthExit` false))))))
  (return (`local.NorthExit`) (`local.SouthExit`) (`local.EastExit`) (`local.WestExit`)))

(fn `UserConstructionScript`)