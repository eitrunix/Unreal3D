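; End-of-level lift that starts the boss fight and serves as the level exit.
; The player gets a widget prompt at the start trigger, and interacting starts a countdown and signals boss start through the game mode.
; Tick runs the timer and, once it expires and the boss-finish event has fired, slides both doors apart with growing per-frame offsets.
; Any overlap with EndLevelTrigger calls the game instance's end-of-level event, without checking actor or state.
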(event `self.ReceiveBeginPlay`
  ;[1 1 1] Dead boss thing
  (bind _astdro_rgame_mode (cast `/Game/TDRoR/Blueprints/GameManagers/TDRoRGameMode` (`GameplayStatics.GetGameMode`)))
  (add `/Game/TDRoR/Blueprints/GameManagers/TDRoRGameMode.OnBossFinish` _astdro_rgame_mode (delegate `BossDead`)))

(event `BossDead`
  ;[1 1 1] Dead boss thing
  (set `self.IsBossDead` true))

(event `self.ReceiveTick`
  (params (DeltaSeconds :type "Float (single-precision)"))
  ;[1 1 1] Check for Level end Trigger to start
  (bind _output_get (set `self.DlltaSeconds` DeltaSeconds))
  (`|ExecutionSequence`
    (:`then_0`
      (if (`self.EndLevelEventStarted`)
        (`self.LevelTimer`)))
    (:`then_1`
      (if (and (`self.OpenDoorBool`) (`self.IsBossDead`))
        (`self.DoorsOpen` _output_get)))))

(event `self.EndLevelTrigger.OnComponentBeginOverlap`
  (params (OverlappedComponent :type "PrimitiveComponent Object Reference") (OtherActor :type "Actor Object Reference") (OtherComp :type "PrimitiveComponent Object Reference") (OtherBodyIndex :type Integer) (bFromSweep :type Boolean) (SweepResult :type "HitResult Structure (by ref)"))
  ;[1 1 1] Player End Level Trigger
  (bind _astdro_rinstance (cast `/Game/TDRoR/Blueprints/GameManagers/TDRoRInstance` (`GameplayStatics.GetGameInstance`)))
  (`/Game/TDRoR/Blueprints/GameManagers/TDRoRInstance.EndOfLevelEvent` _astdro_rinstance))

(event `self.ElevatorStartTrigger.OnComponentBeginOverlap`
  (params (OverlappedComponent :type "PrimitiveComponent Object Reference") (OtherActor :type "Actor Object Reference") (OtherComp :type "PrimitiveComponent Object Reference") (OtherBodyIndex :type Integer) (bFromSweep :type Boolean) (SweepResult :type "HitResult Structure (by ref)"))
  (bind _widget (`self.Widget`))
  ;[1 1 1] Player Interaction
  (cast `/Game/TDRoR/Characters/Heroes/Drongo/DrongoPlayerCharacter` OtherActor)
  (if (not (`self.EndLevelEventStarted`))
    (set `self.Interactable` true)
    (`/Game/TDRoR/Widgets/W_PickUpWidget.Set_CrateText` (cast `/Game/TDRoR/Widgets/W_PickUpWidget` (`WidgetComponent.GetUserWidgetObject` _widget) :!pure true) "Press \"F\" to Interact")
    (`SceneComponent.SetVisibility` _widget true false)))

(event `self.ElevatorStartTrigger.OnComponentEndOverlap`
  (params (OverlappedComponent :type "PrimitiveComponent Object Reference") (OtherActor :type "Actor Object Reference") (OtherComp :type "PrimitiveComponent Object Reference") (OtherBodyIndex :type Integer))
  ;[1 1 1] Player Interaction
  (cast `/Game/TDRoR/Characters/Heroes/Drongo/DrongoPlayerCharacter` OtherActor)
  (if (not (`self.EndLevelEventStarted`))
    (set `self.Interactable` false)
    (`SceneComponent.SetVisibility` (`self.Widget`) false false)))

(event `DoorsOpen`
  (params (`Delta Seconds` :type "Float (double-precision)"))
  (bind _doorposition (`self.DoorPosition`))
  ;[1 1 1] Open Doors of Elevator
  (if (not (`self.DoorTimerFinished`))
    (set `self.DoorPosition` (+ `Delta Seconds` (`self.DoorPosition`)))
    (`SceneComponent.K2_AddRelativeLocation` (`self.Lift01Door01`) (`KismetMathLibrary.MakeVector` _doorposition) false false)
    (`SceneComponent.K2_AddRelativeLocation` (`self.Lift01Door02`) (`KismetMathLibrary.MakeVector` (* _doorposition -1.0)) false false)
    (if (>= (`self.DoorPosition`) (`self.MaxDoorTime`))
      (set `self.DoorTimerFinished` true))))

(event `LevelTimer`
  ;[1 1 1] Wait for Timer to finish, then Open doors. NOTE: Add in Boss Death condition here.
  (if (not (`self.LevelTimerFinished`))
    (set `self.TimerCount` (+ (`self.DlltaSeconds`) (`self.TimerCount`)))
    (if (== (`KismetMathLibrary.FClamp` (* (`self.TimerCount`) 1.0) 0.0 (`self.TimerMax`)) (`self.TimerMax`))
      (set `self.OpenDoorBool` true)
      (set `self.LevelTimerFinished` true))))

(event `ToggleEndLevel`
  ;[1 1 1] Wait for Timer to finish, then Open doors. NOTE: Add in Boss Death condition here.
  (set `self.EndLevelEventStarted` true))

(fn `OnInteract`
  (returns (Success :type Boolean))
  (`self.ToggleEndLevel`)
  (bind _astdro_rgame_mode (cast `/Game/TDRoR/Blueprints/GameManagers/TDRoRGameMode` (`GameplayStatics.GetGameMode`)))
  (`/Game/TDRoR/Blueprints/GameManagers/TDRoRGameMode.OnBossStart` _astdro_rgame_mode)
  (return true))

(fn `UserConstructionScript`
  (bind _lift01door02 (`self.Lift01Door02`))
  (bind _doorposition (`self.DoorPosition`))
  ;[1 1 1] Movement
  (`SceneComponent.K2_AddRelativeLocation` (`self.Lift01Door01`) (`KismetMathLibrary.MakeVector` _doorposition) false false)
  (`SceneComponent.K2_AddRelativeLocation` _lift01door02 (`KismetMathLibrary.MakeVector` (* _doorposition -1.0)) false false)
  ;[1 1 1] Material
  (`PrimitiveComponent.SetMaterial` _lift01door02 0 (`self.Material`))
  (`PrimitiveComponent.SetMaterial` (`self.Lift01Door01`) 0 (`self.Material`)))