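; BP_Lift01_Working is a lift actor that serves as the level exit.
; Its start trigger shows an interact prompt to the TwinStickPawn; ToggleEndLevel, not called here, starts the end-level sequence.
; Tick then runs a countdown, after which both doors slide apart by accumulating relative offsets.
; Overlapping the end trigger opens Level1 and increments the GameInstance stage; the construction script sets initial door offsets and material.
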(event `self.ReceiveBeginPlay`)

(event `self.ReceiveTick`
  (params (DeltaSeconds :type "Float (single-precision)"))
  (bind _output_get (set `self.DlltaSeconds` DeltaSeconds))
  (`|ExecutionSequence`
    (:`then_0`
      (if (`self.EndLevelEventStarted`)
        (`self.LevelTimer`)))
    (:`then_1`
      (if (`self.OpenDoorBool`)
        (`self.DoorsOpen` _output_get)))))

(event `self.EndLevelTrigger.OnComponentBeginOverlap`
  (params (OverlappedComponent :type "PrimitiveComponent Object Reference") (OtherActor :type "Actor Object Reference") (OtherComp :type "PrimitiveComponent Object Reference") (OtherBodyIndex :type Integer) (bFromSweep :type Boolean) (SweepResult :type "HitResult Structure (by ref)"))
  (`GameplayStatics.OpenLevel` "Level1")
  (bind _astdro_rinstance (cast `/Game/TDRoR/GameManagers/TDRoRInstance` (`GameplayStatics.GetGameInstance`)))
  (`/Game/TDRoR/GameManagers/TDRoRInstance.SetStage` _astdro_rinstance (+ (`/Game/TDRoR/GameManagers/TDRoRInstance.currentStage` _astdro_rinstance) 1)))

(event `self.ElevatorStartTrigger.OnComponentBeginOverlap`
  (params (OverlappedComponent :type "PrimitiveComponent Object Reference") (OtherActor :type "Actor Object Reference") (OtherComp :type "PrimitiveComponent Object Reference") (OtherBodyIndex :type Integer) (bFromSweep :type Boolean) (SweepResult :type "HitResult Structure (by ref)"))
  (bind _widget (`self.Widget`))
  (cast `/Game/TwinStickBP/Blueprints/TwinStickPawn` OtherActor)
  (if (not (`self.EndLevelEventStarted`))
    (set `self.Interactable` true)
    (`/Game/TDRoR/Widgets/W_PickUpWidget.Set_CrateText` (cast `/Game/TDRoR/Widgets/W_PickUpWidget` (`WidgetComponent.GetUserWidgetObject` _widget) :!pure true) "Press \"E\" to Interact")
    (`SceneComponent.SetVisibility` _widget true false)))

(event `self.ElevatorStartTrigger.OnComponentEndOverlap`
  (params (OverlappedComponent :type "PrimitiveComponent Object Reference") (OtherActor :type "Actor Object Reference") (OtherComp :type "PrimitiveComponent Object Reference") (OtherBodyIndex :type Integer))
  (cast `/Game/TwinStickBP/Blueprints/TwinStickPawn` OtherActor)
  (if (not (`self.EndLevelEventStarted`))
    (set `self.Interactable` false)
    (`SceneComponent.SetVisibility` (`self.Widget`) false false)))

(event `ToggleEndLevel`
  (set `self.EndLevelEventStarted` true))

(event `DoorsOpen`
  (params (`Delta Seconds` :type "Float (double-precision)"))
  (bind _doorposition (`self.DoorPosition`))
  (bind _doorposition_2 (`self.DoorPosition`))
  (if (not (`self.DoorTimerFinished`))
    (set `self.DoorPosition` (+ `Delta Seconds` _doorposition))
    (`KismetSystemLibrary.PrintString` (`KismetStringLibrary.Conv_DoubleToString` (`KismetMathLibrary.FClamp` (* _doorposition 20.0) 0.0 (`self.MaxDoorTime`))))
    (`SceneComponent.K2_AddRelativeLocation` (`self.Lift01Door01`) (`KismetMathLibrary.MakeVector` _doorposition_2) false false)
    (`SceneComponent.K2_AddRelativeLocation` (`self.Lift01Door02`) (`KismetMathLibrary.MakeVector` (* _doorposition_2 -1.0)) false false)
    (if (>= (`self.DoorPosition`) (`self.MaxDoorTime`))
      (set `self.DoorTimerFinished` true))))

(event `LevelTimer`
  (bind _returnvalue (`KismetMathLibrary.FClamp` (* (`self.TimerCount`) 1.0) 0.0 (`self.TimerMax`)))
  (if (not (`self.LevelTimerFinished`))
    (set `self.TimerCount` (+ (`self.DlltaSeconds`) (`self.TimerCount`)))
    (`KismetSystemLibrary.PrintString` (`KismetStringLibrary.Conv_DoubleToString` _returnvalue))
    (if (== _returnvalue (`self.TimerMax`))
      (set `self.OpenDoorBool` true)
      (set `self.LevelTimerFinished` true))))

(fn `UserConstructionScript`
  (bind _lift01door02 (`self.Lift01Door02`))
  (bind _doorposition (`self.DoorPosition`))
  ;[1 1 1] Movement
  (`SceneComponent.K2_AddRelativeLocation` (`self.Lift01Door01`) (`KismetMathLibrary.MakeVector` _doorposition) false false)
  (`SceneComponent.K2_AddRelativeLocation` _lift01door02 (`KismetMathLibrary.MakeVector` (* _doorposition -1.0)) false false)
  ;[1 1 1] Material
  (`PrimitiveComponent.SetMaterial` _lift01door02 0 (`self.Material`))
  (`PrimitiveComponent.SetMaterial` (`self.Lift01Door01`) 0 (`self.Material`)))